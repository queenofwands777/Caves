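; BloodProbe is a short-lived moving actor that leaves a trail of blood drops behind it.
; Each tick it moves along Direction at Speed with random X/Z jitter and collision sweep, then spawns a BloodDrop and a BloodDropSmall at randomly offset nearby points.
; Lifetime counts down in ticks rather than seconds, destroying the probe at zero.
; The Splatter function is an empty stub.
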(event EventBeginPlay)

(event EventTick
  (params (DeltaSeconds :type Float%20%28single-precision%29))
  (Transformation|AddActorWorldOffset (+ (Math|Vector|MakeVector (Math|Random|RandomFloatinRange -2.0 2.0) 0.0 (Math|Random|RandomFloatinRange -2.0 2.0)) (* DeltaSeconds (* (Variables|Default|GetDirection) (Variables|Default|GetSpeed)))) true)
  (Game|SpawnActorfromClass "/Game/Blueprints/BloodDrop.BloodDrop_C" (Math|Transform|MakeTransform (+ (Transformation|GetActorLocation) (Math|Vector|MakeVector (Math|Random|RandomFloatinRange -5.0 5.0) 0.0 (Math|Random|RandomFloatinRange -5.0 5.0)))) "Undefined" "MultiplyWithRoot" 0 0)
  (Game|SpawnActorfromClass "/Game/Blueprints/BloodDropSmall.BloodDropSmall_C" (Math|Transform|MakeTransform (+ (Transformation|GetActorLocation) (Math|Vector|MakeVector (Math|Random|RandomFloatinRange -5.0 5.0) 0.0 (Math|Random|RandomFloatinRange -5.0 5.0)))) "Undefined" "MultiplyWithRoot" 0 0)
  (Variables|Default|SetLifetime (- (Variables|Default|GetLifetime) 1))
  (if (<= (Variables|Default|GetLifetime) 0)
    (Actor|DestroyActor)))

(fn ConstructionScript)

(fn Splatter
  (params (direction :type Vector) (num_probes :type Integer) (max_angle :type Float%20%28double-precision%29)))