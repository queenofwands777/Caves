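; Player actor that moves in the X-Z plane and fires TrailBullet projectiles toward the mouse cursor.
; Up and Left axis input accumulates until Tick, where CustomMove applies a swept world offset and stops CharacterMovement on a blocking hit.
; Aim comes from the viewport vector between projected actor position and cursor, setting Gun pitch each frame.
; Fire spawns a bullet slightly offset along that direction, with screen Y flipped for world Z.
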(event EventBeginPlay)

(event Collision|EventActorBeginOverlap
  (params (OtherActor :type Actor%20Object%20Reference)))

(event EventTick
  (params (DeltaSeconds :type Float%20%28single-precision%29))
  (CallFunction|CustomMove (Variables|Default|GetUpDown) (Variables|Default|GetLeftRight) DeltaSeconds)
  (Variables|Default|SetUpDown 0.0)
  (Variables|Default|SetLeftRight 0.0)
  (bind _returnvalue (Class|WidgetLayoutLibrary|GetMousePositiononViewport))
  (Transformation|SetRelativeRotation (Variables|Default|Getgun) (Math|Rotator|MakeRotator 0.0 (* (Class|KismetMathLibrary|DegAsin (Math|Vector|DotProduct (Math|Vector|MakeVector (.X (Math|Vector|BreakVector (Math|Vector|Normalize (Math|Conversions|ToVector(Vector2D) (- _returnvalue (Class|SlateBlueprintLibrary|ScreentoViewport (.ScreenPosition (Class|GameplayStatics|ProjectWorldtoScreen (Game|GetPlayerController 0) (Transformation|GetActorLocation) false)))))))) 0.0 (.Y (Math|Vector|BreakVector (Math|Vector|Normalize (Math|Conversions|ToVector(Vector2D) (- _returnvalue (Class|SlateBlueprintLibrary|ScreentoViewport (.ScreenPosition (Class|GameplayStatics|ProjectWorldtoScreen (Game|GetPlayerController 0) (Transformation|GetActorLocation) false))))))))) "1.000000,0.000000,0.000000")) (Math|Float|Sign(Float) (.Y (Math|Vector|BreakVector (Math|Vector|Normalize (Math|Conversions|ToVector(Vector2D) (- _returnvalue (Class|SlateBlueprintLibrary|ScreentoViewport (.ScreenPosition (Class|GameplayStatics|ProjectWorldtoScreen (Game|GetPlayerController 0) (Transformation|GetActorLocation) false)))))))))) 0.0) false false))

(event Input|ActionEvents|InputActionFire
  (params (Key :type Key%20Structure :default "None"))
  (bind _returnvalue (Transformation|GetActorTransform))
  (bind (_location _rotation _scale) (Math|Transform|BreakTransform _returnvalue))
  (bind (_x _y _z) (Math|Vector|BreakVector _location))
  (:Pressed
    (bind _returnvalue_2 (Class|WidgetLayoutLibrary|GetMousePositiononViewport))
    (Game|SpawnActorfromClass "/Game/Blueprints/TrailBullet.TrailBullet_C" (Math|Transform|MakeTransform (Math|Vector|MakeVector (+ (* 0.5 (.X (Math|Vector2D|BreakVector2D (* (Math|Conversions|ToVector2D(Vector) (Math|Vector|Normalize (Math|Conversions|ToVector(Vector2D) (- _returnvalue_2 (Class|SlateBlueprintLibrary|ScreentoViewport (.ScreenPosition (Class|GameplayStatics|ProjectWorldtoScreen (Game|GetPlayerController 0) (Transformation|GetActorLocation) false))))))) (Math|Vector2D|MakeVector2D 1.0 -1.0))))) _x) _y (+ (* 0.5 (.Y (Math|Vector2D|BreakVector2D (* (Math|Conversions|ToVector2D(Vector) (Math|Vector|Normalize (Math|Conversions|ToVector(Vector2D) (- _returnvalue_2 (Class|SlateBlueprintLibrary|ScreentoViewport (.ScreenPosition (Class|GameplayStatics|ProjectWorldtoScreen (Game|GetPlayerController 0) (Transformation|GetActorLocation) false))))))) (Math|Vector2D|MakeVector2D 1.0 -1.0))))) _z)) _rotation _scale) "Undefined" "MultiplyWithRoot" 0 (* (Math|Conversions|ToVector2D(Vector) (Math|Vector|Normalize (Math|Conversions|ToVector(Vector2D) (- _returnvalue_2 (Class|SlateBlueprintLibrary|ScreentoViewport (.ScreenPosition (Class|GameplayStatics|ProjectWorldtoScreen (Game|GetPlayerController 0) (Transformation|GetActorLocation) false))))))) (Math|Vector2D|MakeVector2D 1.0 -1.0)) 0)))

(event Input|AxisEvents|InputAxisUp
  (params (AxisValue :type Float%20%28single-precision%29))
  (Variables|Default|SetUpDown (+ AxisValue (Variables|Default|GetUpDown))))

(event Input|AxisEvents|InputAxisLeft
  (params (AxisValue :type Float%20%28single-precision%29))
  (Variables|Default|SetLeftRight (+ AxisValue (Variables|Default|GetLeftRight))))

(fn ConstructionScript)

(fn CustomMove
  (params (UpDown :type Float%20%28double-precision%29) (LeftRight :type Float%20%28double-precision%29) (DeltaTime :type Float%20%28double-precision%29))
  (bind _sweephitresult (Transformation|AddActorWorldOffset (* (* (Variables|Default|GetSpeed) DeltaTime) (Math|Vector|MakeVector LeftRight 0.0 UpDown)) true))
  (if (.bBlockingHit (Collision|BreakHitResult _sweephitresult))
    (Class|NavMovementComponent|StopActiveMovement (Variables|Character|GetCharacterMovement))))