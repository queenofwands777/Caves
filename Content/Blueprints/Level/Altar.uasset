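; Altar level actor that offers a random perk when play begins.
; On BeginPlay it casts the game instance to GameVar and picks a random class from its PerksRemaining array.
; It spawns that class slightly offset above the altar, matching its rotation and scale, and leaves the array unchanged.
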(event EventBeginPlay
  (bind _returnvalue (Transformation|GetActorTransform))
  (bind (_location _rotation _scale) (Math|Transform|BreakTransform _returnvalue))
  (bind (_x _y _z) (Math|Vector|BreakVector _location))
  (bind _asgame_var (Utilities|Casting|CastToGameVar (Game|GetGameInstance)))
  (Game|SpawnActorfromClass (Utilities|Array|Get(acopy) (Variables|/Game/Blueprints/Engine/GameVar.GameVar_C|GetPerksRemaining _asgame_var) (Math|Random|RandomInteger (Utilities|Array|Length (Variables|/Game/Blueprints/Engine/GameVar.GameVar_C|GetPerksRemaining _asgame_var)))) (Math|Transform|MakeTransform (Math|Vector|MakeVector _x (+ _y 1.0) (+ 7.0 _z)) _rotation _scale) "Undefined" "MultiplyWithRoot" 0 0))

(event Collision|EventActorBeginOverlap
  (params (OtherActor :type Actor%20Object%20Reference)))

(event EventTick
  (params (DeltaSeconds :type Float%20%28single-precision%29)))

(fn ConstructionScript)