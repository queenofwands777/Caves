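; Level exit portal that opens once every enemy is gone and moves the game on to a new level.
; Tick polls for remaining Enemy actors, and when none are left the portal swaps to its open sprite and sets the Open flag.
; Player overlap with the sprite prints whether the level is complete and, if open, has the TopDown game mode clear and regenerate the level.
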(event OnComponentBeginOverlap(PaperSprite)
  (params (OverlappedComponent :type Primitive%20Component%20Object%20Reference) (OtherActor :type Actor%20Object%20Reference) (OtherComp :type Primitive%20Component%20Object%20Reference) (OtherBodyIndex :type Integer) (bFromSweep :type Boolean) (SweepResult :type Hit%20Result%20Structure%20%28by%20ref%29))
  (Utilities|Casting|CastToplayer OtherActor)
  (if (Variables|Default|GetOpen)
    (Development|PrintText "LEVEL COMPLETE")
    (bind _astop_down (Utilities|Casting|CastToTopDown (Game|GetGameMode)))
    (Default|ClearLevel _astop_down)
    (Default|GenerateLevel _astop_down)
    (else
      (Development|PrintText "LEVEL INCOMPLETE"))))

(event EventTick
  (params (DeltaSeconds :type Float%20%28single-precision%29))
  (bind _outactors (Actor|GetAllActorsOfClass "/Game/Blueprints/Entities/enemy.enemy_C"))
  (if (Math|Conversions|ToBoolean(Integer) (Class|KismetMathLibrary|AndIntInt (Math|Conversions|ToInteger(Boolean) (== (Utilities|Array|Length _outactors) 0)) (Math|Conversions|ToInteger(Boolean) (not (Variables|Default|GetOpen)))))
    (CallFunction|OpenPortal)))

(fn ConstructionScript)

(fn OpenPortal
  (Rendering|Components|Sprite|SetSprite (Variables|Default|GetPaperSprite) "/Game/Assets/Level/PortalOpen1_Sprite.PortalOpen1_Sprite")
  (Variables|Default|SetOpen true))