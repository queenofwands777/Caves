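; Enemy entity Blueprint that equips a weapon and seeds randomized movement on spawn, extending a parent class.
; BeginPlay sets the sprite and selection on its first Weapon component, then picks a random move threshold and a nearby target in the XZ plane.
; Capsule hits negate the target's absolute X and Z coordinates and zero Y.
; Tick only calls the parent, so no movement toward the target happens in this graph.
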(event OnComponentHit(CapsuleComponent)
  (params (HitComponent :type Primitive%20Component%20Object%20Reference) (OtherActor :type Actor%20Object%20Reference) (OtherComp :type Primitive%20Component%20Object%20Reference) (NormalImpulse :type Vector :default "0, 0, 0") (Hit :type Hit%20Result%20Structure%20%28by%20ref%29))
  (Variables|Default|SetTargetDestination (* "-1.000000,0.000000,-1.000000" (Variables|Default|GetTargetDestination))))

(event EventBeginPlay
  (bind _returnvalue (Actor|GetComponentsByClass "/Game/Blueprints/Weapons/Weapon.Weapon_C"))
  (bind _returnvalue_2 (Transformation|GetActorLocation))
  (bind (_x _y _z) (Math|Vector|BreakVector _returnvalue_2))
  (bind _output (Utilities|Array|Get(acopy) _returnvalue))
  (|CallParentFunction)
  (if (> (Utilities|Array|Length _returnvalue) 0)
    (Default|SetSprite _output)
    (Default|SelectWeapon _output))
  ;[1 1 1] Init movement
  (Variables|Default|SetMoveThreshold (Math|Conversions|ToFloat(Integer) (Math|Random|RandomIntegerinRange 60 300)))
  (Variables|Default|SetTargetDestination (Math|Vector|MakeVector (+ (Math|Random|RandomFloatinRange -2e+01 2e+01) _x) _y (+ _z (Math|Random|RandomFloatinRange -2e+01 2e+01)))))

(event EventTick
  (params (DeltaSeconds :type Float%20%28single-precision%29))
  (|CallParentFunction DeltaSeconds))

(fn ConstructionScript)