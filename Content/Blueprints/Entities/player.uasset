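; Player character for a top-down 2D shooter that moves on the XZ plane, aims at the mouse and fires a weapon component.
; Tick applies swept movement, rotates hand and sprite, offsets the camera arm logarithmically toward the cursor and updates the HUD.
; GameVar and HelpfulGhost carry stats, weapon and perks between spawns; destruction when dead resets weapon and perks and ends the game.
; Weapon-cycling logic is disconnected.
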(event EventBeginPlay
  ;[1 1 1] Begin Play
  ;;[1 1 1] Load Run State
  (Variables|Default|SetAdvancing false)
  (bind _asgame_var (Utilities|Casting|CastToGameVar (Game|GetGameInstance)))
  (Variables|Default|SetHealth (Variables|/Game/Blueprints/Engine/GameVar.GameVar_C|GetPlayerHealth _asgame_var))
  (Variables|Default|SetAmmo (Variables|/Game/Blueprints/Engine/GameVar.GameVar_C|GetPlayerAmmo _asgame_var))
  (Game|AddComponentbyClass (Variables|/Game/Blueprints/Engine/GameVar.GameVar_C|GetWeapon _asgame_var))
  (bind _returnvalue (Actor|GetActorOfClass "/Game/Blueprints/Engine/HelpfulGhost.HelpfulGhost_C"))
  (Default|SendPerksGhosttoPlayer _returnvalue self)
  ;;[1 1 1] initialize hud values
  (bind _foundwidgets (Widget|GetAllWidgetsOfClass "/Game/Blueprints/UI/HUD.HUD_C" true))
  (for _array_element _foundwidgets
    (Variables|/Game/Blueprints/UI/HUD.HUD_C|SetPlayerHealth _array_element (Variables|Default|GetHealth))
    (Variables|/Game/Blueprints/UI/HUD.HUD_C|SetPlayerAmmo _array_element (Variables|Default|GetAmmo))
    (Variables|/Game/Blueprints/UI/HUD.HUD_C|SetPlayerMaxHealth _array_element (Variables|/Game/Blueprints/Engine/GameVar.GameVar_C|GetPlayerMaxHealth _asgame_var))))

(event EventDestroyed
  (if (Variables|Default|GetAlive)
    ;[1 1 1] Destructor
    (bind _asgame_var (Utilities|Casting|CastToGameVar (Game|GetGameInstance)))
    (Variables|/Game/Blueprints/Engine/GameVar.GameVar_C|SetPlayerHealth _asgame_var (Variables|Default|GetHealth))
    (Variables|/Game/Blueprints/Engine/GameVar.GameVar_C|SetPlayerAmmo _asgame_var (Variables|Default|GetAmmo))
    (Variables|/Game/Blueprints/Engine/GameVar.GameVar_C|SetWeapon _asgame_var (Utilities|GetClass (Actor|GetComponentbyClass "/Game/Blueprints/Weapons/Weapon.Weapon_C")))
    (for _array_element (Actor|GetComponentsByClass self "/Game/Blueprints/Perks/Perk.Perk_C")
      (bind _returnvalue (Actor|GetActorOfClass "/Game/Blueprints/Engine/HelpfulGhost.HelpfulGhost_C"))
      (Default|SendPerkPlayertoGhost _returnvalue (Utilities|GetClass _array_element)))
    (else
      (bind _astop_down (Utilities|Casting|CastToTopDown (Game|GetGameMode)))
      (bind _asgame_var_2 (Utilities|Casting|CastToGameVar (Game|GetGameInstance)))
      (Variables|/Game/Blueprints/Engine/GameVar.GameVar_C|SetWeapon _asgame_var_2 "/Game/Blueprints/Weapons/Ranged/Pistol.Pistol_C")
      (bind _returnvalue_2 (Actor|GetActorOfClass "/Game/Blueprints/Engine/HelpfulGhost.HelpfulGhost_C"))
      (Default|RemovePerks _returnvalue_2)
      (bind _asgame_var_3 (Utilities|Casting|CastToGameVar (Game|GetGameInstance)))
      (Variables|/Game/Blueprints/Engine/GameVar.GameVar_C|SetPerksRemaining _asgame_var_3 (Variables|/Game/Blueprints/Engine/GameVar.GameVar_C|GetPerks _asgame_var_3))
      (Default|EndGame _astop_down))))

(event EventTick
  (params (DeltaSeconds :type Float%20%28single-precision%29))
  (bind _hand (Variables|Default|Gethand))
  (bind _returnvalue (Components|GetChildComponent _hand 0))
  (|CallParentFunction DeltaSeconds)
  ;[1 1 1] Tick
  ;;[1 1 1] Player Movement
  (if (not (Variables|Default|GetAdvancing))
    (CallFunction|CustomMove (Variables|Default|GetUpDown) (Variables|Default|GetLeftRight) DeltaSeconds)
    (Variables|Default|SetUpDown 0.0)
    (Variables|Default|SetLeftRight 0.0)
    ;;[1 1 1] Weapon rotation
    (bind _returnvalue_2 (Class|WidgetLayoutLibrary|GetMousePositiononViewport))
    (Variables|Default|SetPointDirection (* (Math|Vector|MakeVector (.X (Math|Vector|BreakVector (Math|Vector|Normalize (Math|Conversions|ToVector(Vector2D) (- _returnvalue_2 (Class|SlateBlueprintLibrary|ScreentoViewport (.ScreenPosition (Class|GameplayStatics|ProjectWorldtoScreen (Game|GetPlayerController 0) (Transformation|GetActorLocation) false)))))))) 0.0 (.Y (Math|Vector|BreakVector (Math|Vector|Normalize (Math|Conversions|ToVector(Vector2D) (- _returnvalue_2 (Class|SlateBlueprintLibrary|ScreentoViewport (.ScreenPosition (Class|GameplayStatics|ProjectWorldtoScreen (Game|GetPlayerController 0) (Transformation|GetActorLocation) false))))))))) (Math|Vector|MakeVector 1.0 0.0 -1.0)))
    (Transformation|SetRelativeRotation _returnvalue (Math|Rotator|MakeRotator (+ (* (Math|Float|Sign(Float) (.X (Math|Vector|BreakVector (Math|Vector|Normalize (Math|Conversions|ToVector(Vector2D) (- _returnvalue_2 (Class|SlateBlueprintLibrary|ScreentoViewport (.ScreenPosition (Class|GameplayStatics|ProjectWorldtoScreen (Game|GetPlayerController 0) (Transformation|GetActorLocation) false))))))))) 9e+01) 9e+01) (+ (+ (* (Math|Float|Sign(Float) (.X (Math|Vector|BreakVector (Math|Vector|Normalize (Math|Conversions|ToVector(Vector2D) (- _returnvalue_2 (Class|SlateBlueprintLibrary|ScreentoViewport (.ScreenPosition (Class|GameplayStatics|ProjectWorldtoScreen (Game|GetPlayerController 0) (Transformation|GetActorLocation) false))))))))) 9e+01) 9e+01) (+ (* (Class|KismetMathLibrary|DegAsin (Math|Vector|DotProduct (Math|Vector|MakeVector (.X (Math|Vector|BreakVector (Math|Vector|Normalize (Math|Conversions|ToVector(Vector2D) (- _returnvalue_2 (Class|SlateBlueprintLibrary|ScreentoViewport (.ScreenPosition (Class|GameplayStatics|ProjectWorldtoScreen (Game|GetPlayerController 0) (Transformation|GetActorLocation) false)))))))) 0.0 (.Y (Math|Vector|BreakVector (Math|Vector|Normalize (Math|Conversions|ToVector(Vector2D) (- _returnvalue_2 (Class|SlateBlueprintLibrary|ScreentoViewport (.ScreenPosition (Class|GameplayStatics|ProjectWorldtoScreen (Game|GetPlayerController 0) (Transformation|GetActorLocation) false))))))))) "1.000000,0.000000,0.000000")) (Math|Float|Sign(Float) (.Y (Math|Vector|BreakVector (Math|Vector|Normalize (Math|Conversions|ToVector(Vector2D) (- _returnvalue_2 (Class|SlateBlueprintLibrary|ScreentoViewport (.ScreenPosition (Class|GameplayStatics|ProjectWorldtoScreen (Game|GetPlayerController 0) (Transformation|GetActorLocation) false)))))))))) (+ (* (Math|Float|Sign(Float) (.Y (Math|Vector|BreakVector (Math|Vector|Normalize (Math|Conversions|ToVector(Vector2D) (- _returnvalue_2 (Class|SlateBlueprintLibrary|ScreentoViewport (.ScreenPosition (Class|GameplayStatics|ProjectWorldtoScreen (Game|GetPlayerController 0) (Transformation|GetActorLocation) false))))))))) 9e+01) 9e+01))) 0.0) false false)
    (Transformation|SetRelativeRotation (Variables|Default|GetSprite) (Math|Rotator|MakeRotator 0.0 0.0 (+ (* (Math|Float|Sign(Float) (.X (Math|Vector|BreakVector (Math|Vector|Normalize (Math|Conversions|ToVector(Vector2D) (- _returnvalue_2 (Class|SlateBlueprintLibrary|ScreentoViewport (.ScreenPosition (Class|GameplayStatics|ProjectWorldtoScreen (Game|GetPlayerController 0) (Transformation|GetActorLocation) false))))))))) 9e+01) 9e+01)) false false)
    (Variables|Default|SetFacingLeft (== (+ (* (Math|Float|Sign(Float) (.X (Math|Vector|BreakVector (Math|Vector|Normalize (Math|Conversions|ToVector(Vector2D) (- _returnvalue_2 (Class|SlateBlueprintLibrary|ScreentoViewport (.ScreenPosition (Class|GameplayStatics|ProjectWorldtoScreen (Game|GetPlayerController 0) (Transformation|GetActorLocation) false))))))))) 9e+01) 9e+01) 0.0))
    (Transformation|SetRelativeLocation _returnvalue (Math|Vector|MakeVector (* (.X (Math|Vector|BreakVector (Math|Vector|MakeVector (.X (Math|Vector|BreakVector (Math|Vector|Normalize (Math|Conversions|ToVector(Vector2D) (- _returnvalue_2 (Class|SlateBlueprintLibrary|ScreentoViewport (.ScreenPosition (Class|GameplayStatics|ProjectWorldtoScreen (Game|GetPlayerController 0) (Transformation|GetActorLocation) false)))))))) 0.0 (.Y (Math|Vector|BreakVector (Math|Vector|Normalize (Math|Conversions|ToVector(Vector2D) (- _returnvalue_2 (Class|SlateBlueprintLibrary|ScreentoViewport (.ScreenPosition (Class|GameplayStatics|ProjectWorldtoScreen (Game|GetPlayerController 0) (Transformation|GetActorLocation) false))))))))))) 1e+01) 1.0 (* (* (.Z (Math|Vector|BreakVector (Math|Vector|MakeVector (.X (Math|Vector|BreakVector (Math|Vector|Normalize (Math|Conversions|ToVector(Vector2D) (- _returnvalue_2 (Class|SlateBlueprintLibrary|ScreentoViewport (.ScreenPosition (Class|GameplayStatics|ProjectWorldtoScreen (Game|GetPlayerController 0) (Transformation|GetActorLocation) false)))))))) 0.0 (.Y (Math|Vector|BreakVector (Math|Vector|Normalize (Math|Conversions|ToVector(Vector2D) (- _returnvalue_2 (Class|SlateBlueprintLibrary|ScreentoViewport (.ScreenPosition (Class|GameplayStatics|ProjectWorldtoScreen (Game|GetPlayerController 0) (Transformation|GetActorLocation) false))))))))))) 1e+01) -1.0)) false false)
    ;;[1 1 1] Update HUD
    (bind _foundwidgets (Widget|GetAllWidgetsOfClass "/Game/Blueprints/UI/HUD.HUD_C" true))
    (for _array_element _foundwidgets
      (Variables|/Game/Blueprints/UI/HUD.HUD_C|SetPlayerHealth _array_element (Variables|Default|GetHealth))
      (Variables|/Game/Blueprints/UI/HUD.HUD_C|SetPlayerAmmo _array_element (Variables|Default|GetAmmo))
      (Transformation|SetRelativeLocation (Variables|Default|GetSpringArm) (* (* (Variables|Default|GetPointDirection) 5.0) (Math|Float|Log (Math|Vector|VectorLengthXY (Math|Conversions|ToVector(Vector2D) (- _returnvalue_2 (Class|SlateBlueprintLibrary|ScreentoViewport (.ScreenPosition (Class|GameplayStatics|ProjectWorldtoScreen (Game|GetPlayerController 0) (Transformation|GetActorLocation) false)))))) 1e+02)) false false))))

(event Input|ActionEvents|InputActionInteract
  (params (Key :type Key%20Structure :default "None"))
  (:Pressed
    (Variables|Default|SetInteracting true)
    (Development|PrintText "Player is interacting"))
  (:Released
    (Variables|Default|SetInteracting false)))

(event Input|ActionEvents|InputActionFire
  (params (Key :type Key%20Structure :default "None"))
  (bind _returnvalue (Actor|GetComponentbyClass "/Game/Blueprints/Weapons/Weapon.Weapon_C"))
  ;[1 1 1] Fire Weapon
  (:Pressed
    (if (> (Variables|Default|GetAmmo) 0)
      (Default|SetFire _returnvalue)))
  (:Released
    (Default|EndFire _returnvalue)))

(event Input|AxisEvents|InputAxisUp
  (params (AxisValue :type Float%20%28single-precision%29))
  ;[1 1 1] Set Player Movement
  (if true
    (Variables|Default|SetUpDown (+ AxisValue (Variables|Default|GetUpDown)))))

(event Input|AxisEvents|InputAxisLeft
  (params (AxisValue :type Float%20%28single-precision%29))
  ;[1 1 1] Set Player Movement
  (if true
    (Variables|Default|SetLeftRight (+ AxisValue (Variables|Default|GetLeftRight)))))

(event Input|AxisEvents|InputAxisSwitch
  (params (AxisValue :type Float%20%28single-precision%29))
  ;[1 1 1] Switch Weapon
)

(fn ConstructionScript)

(fn CustomMove
  (params (UpDown :type Float%20%28double-precision%29) (LeftRight :type Float%20%28double-precision%29) (DeltaTime :type Float%20%28double-precision%29))
  (if (or (!= UpDown 0.0) (!= LeftRight 0.0))
    (if (or (and (== LeftRight 1.0) (Variables|Default|GetFacingLeft)) (and (== LeftRight -1.0) (not (Variables|Default|GetFacingLeft))))
      (Variables|Default|SetMoving true)
      (Variables|Default|SetMovingBackwards true)
      (else
        (Variables|Default|SetMoving true)
        (Variables|Default|SetMovingBackwards false)))
    (else
      (Variables|Default|SetMoving false)
      (Variables|Default|SetMovingBackwards false)))
  (bind _sweephitresult (Transformation|AddActorWorldOffset (* (* (* (Variables|Default|GetSpeedMultiplier) (Variables|Default|GetSpeed)) DeltaTime) (Math|Vector|MakeVector LeftRight 0.0 UpDown)) true))
  (if (.bBlockingHit (Collision|BreakHitResult _sweephitresult))
    (Class|NavMovementComponent|StopActiveMovement (Variables|Character|GetCharacterMovement))))

(fn SwitchWeapon
  (params (NewParam :type Weapon%20Class%20Reference))
  (Components|DestroyComponent (Actor|GetComponentbyClass "/Game/Blueprints/Weapons/Weapon.Weapon_C"))
  (Components|DestroyComponent (Components|GetChildComponent (Variables|Default|Gethand) 0))
  (Game|AddComponentbyClass NewParam))

(fn SetAnimation
  (bind _sprite (Variables|Default|GetSprite))
  (if (Variables|Default|GetMoving)
    (if (Variables|Default|GetMovingBackwards)
      (Sprite|SetFlipbook _sprite "/Game/Assets/Entities/Character/Walk/CharacterWalkBackwards.CharacterWalkBackwards")
      (else
        (Sprite|SetFlipbook _sprite "/Game/Assets/Entities/Character/Walk/CharacterWalk.CharacterWalk")))
    (else
      (Sprite|SetFlipbook _sprite "/Game/Assets/Entities/Character/Idle/CharacterIdle.CharacterIdle"))))