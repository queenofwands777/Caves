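; Arms component that builds and animates procedural 2D Paper2D arms for an Entity holding a weapon.
; BeginPlay spawns tinted shoulder, bicep, elbow, forearm and hand sprites for both sides.
; Tick pins hands to the Weapon's hold points, solves elbows with equal-length two-bone IK, then aligns limb segments between joints.
; PointDirection's X sign flips the body, weapon, elbow bend and depth offsets; left-arm solving is skipped for one-handed weapons.
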(event EventBeginPlay
  (bind _returnvalue (Components|GetOwner))
  (bind _returnvalue_2 (Components|GetOwner))
  (bind _asentity (Utilities|Casting|CastToEntity _returnvalue))
  (bind _handcolor (Variables|/Game/Blueprints/Entities/Entity.Entity_C|GetHandColor _asentity))
  (bind _leftarmcolor (Variables|/Game/Blueprints/Entities/Entity.Entity_C|GetLeftArmColor _asentity))
  (bind _rightarmcolor (Variables|/Game/Blueprints/Entities/Entity.Entity_C|GetRightArmColor _asentity))
  ;[1 1 1] Initialize Sprites
  (if true
    (bind _returnvalue_3 (Game|AddComponentbyClass _returnvalue_2 "/Script/Paper2D.PaperSpriteComponent" false))
    (Collision|SetCollisionEnabled _returnvalue_3 "NoCollision")
    (Sprite|SetSpriteColor _returnvalue_3 _rightarmcolor)
    (Rendering|Components|Sprite|SetSprite _returnvalue_3 "/Game/Assets/Entities/Arm/ArmJoint1_Sprite.ArmJoint1_Sprite")
    (Variables|Default|SetRightShoulderSprite _returnvalue_3)
    (bind _returnvalue_4 (Game|AddComponentbyClass _returnvalue_2 "/Script/Paper2D.PaperSpriteComponent" false))
    (Collision|SetCollisionEnabled _returnvalue_4 "NoCollision")
    (Sprite|SetSpriteColor _returnvalue_4 _rightarmcolor)
    (Rendering|Components|Sprite|SetSprite _returnvalue_4 "/Game/Assets/Entities/Arm/ArmPart1_Sprite.ArmPart1_Sprite")
    (Variables|Default|SetRightBicepSprite _returnvalue_4)
    (bind _returnvalue_5 (Game|AddComponentbyClass _returnvalue_2 "/Script/Paper2D.PaperSpriteComponent" false))
    (Collision|SetCollisionEnabled _returnvalue_5 "NoCollision")
    (Sprite|SetSpriteColor _returnvalue_5 _rightarmcolor)
    (Rendering|Components|Sprite|SetSprite _returnvalue_5 "/Game/Assets/Entities/Arm/ArmJoint1_Sprite.ArmJoint1_Sprite")
    (Variables|Default|SetRightElbowSprite _returnvalue_5)
    (bind _returnvalue_6 (Game|AddComponentbyClass _returnvalue_2 "/Script/Paper2D.PaperSpriteComponent" false))
    (Collision|SetCollisionEnabled _returnvalue_6 "NoCollision")
    (Sprite|SetSpriteColor _returnvalue_6 _rightarmcolor)
    (Rendering|Components|Sprite|SetSprite _returnvalue_6 "/Game/Assets/Entities/Arm/ArmPart1_Sprite.ArmPart1_Sprite")
    (Variables|Default|SetRightForearmSprite _returnvalue_6)
    (bind _returnvalue_7 (Game|AddComponentbyClass _returnvalue_2 "/Script/Paper2D.PaperSpriteComponent" false))
    (Collision|SetCollisionEnabled _returnvalue_7 "NoCollision")
    (Sprite|SetSpriteColor _returnvalue_7 _handcolor)
    (Rendering|Components|Sprite|SetSprite _returnvalue_7 "/Game/Assets/Entities/Arm/ArmJoint1_Sprite.ArmJoint1_Sprite")
    (Variables|Default|SetRightHandSprite _returnvalue_7)
    (bind _returnvalue_8 (Game|AddComponentbyClass _returnvalue_2 "/Script/Paper2D.PaperSpriteComponent" false))
    (Collision|SetCollisionEnabled _returnvalue_8 "NoCollision")
    (Sprite|SetSpriteColor _returnvalue_8 _leftarmcolor)
    (Rendering|Components|Sprite|SetSprite _returnvalue_8 "/Game/Assets/Entities/Arm/ArmJoint1_Sprite.ArmJoint1_Sprite")
    (Variables|Default|SetLeftShoulderSprite _returnvalue_8)
    (bind _returnvalue_9 (Game|AddComponentbyClass _returnvalue_2 "/Script/Paper2D.PaperSpriteComponent" false))
    (Collision|SetCollisionEnabled _returnvalue_9 "NoCollision")
    (Sprite|SetSpriteColor _returnvalue_9 _leftarmcolor)
    (Rendering|Components|Sprite|SetSprite _returnvalue_9 "/Game/Assets/Entities/Arm/ArmPart1_Sprite.ArmPart1_Sprite")
    (Variables|Default|SetLeftBicepSprite _returnvalue_9)
    (bind _returnvalue_10 (Game|AddComponentbyClass _returnvalue_2 "/Script/Paper2D.PaperSpriteComponent" false))
    (Collision|SetCollisionEnabled _returnvalue_10 "NoCollision")
    (Sprite|SetSpriteColor _returnvalue_10 _leftarmcolor)
    (Rendering|Components|Sprite|SetSprite _returnvalue_10 "/Game/Assets/Entities/Arm/ArmJoint1_Sprite.ArmJoint1_Sprite")
    (Variables|Default|SetLeftElbowSprite _returnvalue_10)
    (bind _returnvalue_11 (Game|AddComponentbyClass _returnvalue_2 "/Script/Paper2D.PaperSpriteComponent" false))
    (Collision|SetCollisionEnabled _returnvalue_11 "NoCollision")
    (Sprite|SetSpriteColor _returnvalue_11 _leftarmcolor)
    (Rendering|Components|Sprite|SetSprite _returnvalue_11 "/Game/Assets/Entities/Arm/ArmPart1_Sprite.ArmPart1_Sprite")
    (Variables|Default|SetLeftForearmSprite _returnvalue_11)
    (bind _returnvalue_12 (Game|AddComponentbyClass _returnvalue_2 "/Script/Paper2D.PaperSpriteComponent" false))
    (Collision|SetCollisionEnabled _returnvalue_12 "NoCollision")
    (Sprite|SetSpriteColor _returnvalue_12 _handcolor)
    (Rendering|Components|Sprite|SetSprite _returnvalue_12 "/Game/Assets/Entities/Arm/ArmJoint1_Sprite.ArmJoint1_Sprite")
    (Variables|Default|SetLeftHandSprite _returnvalue_12)))

(event EventTick
  (params (DeltaSeconds :type Float%20%28single-precision%29))
  (bind _returnvalue (Components|GetOwner))
  (bind _returnvalue_2 (Components|GetOwner))
  (bind _returnvalue_3 (Components|GetOwner))
  (bind _returnvalue_4 (Components|GetOwner))
  (bind _returnvalue_5 (Components|GetOwner))
  (bind _asentity (Utilities|Casting|CastToEntity _returnvalue_2))
  (bind _asentity_2 (Utilities|Casting|CastToEntity _returnvalue))
  (bind _asentity_3 (Utilities|Casting|CastToEntity _returnvalue_3))
  (bind _asentity_4 (Utilities|Casting|CastToEntity _returnvalue_5))
  (bind _asentity_5 (Utilities|Casting|CastToEntity _returnvalue_4))
  (bind _returnvalue_6 (Actor|GetComponentbyClass _asentity_2 "/Game/Blueprints/Weapons/Weapon.Weapon_C"))
  (bind _returnvalue_7 (Actor|GetComponentsbyTag _asentity "/Script/Engine.SpringArmComponent" "hand"))
  (bind _returnvalue_8 (Actor|GetComponentbyClass _asentity_5 "/Game/Blueprints/Weapons/Weapon.Weapon_C"))
  (bind _returnvalue_9 (Actor|GetComponentsbyTag _asentity_4 "/Script/Engine.SpringArmComponent" "hand"))
  (bind _pointdirection (Variables|/Game/Blueprints/Entities/Entity.Entity_C|GetPointDirection _asentity_3))
  (bind _x (Math|Vector|BreakVector _pointdirection))
  (bind _output (Utilities|Array|Get(acopy) _returnvalue_7))
  (bind _output_2 (Utilities|Array|Get(acopy) _returnvalue_9))
  (bind _lefthandhold (Variables|/Game/Blueprints/Weapons/Weapon.Weapon_C|GetLeftHandHold _returnvalue_8))
  (bind _righthandhold (Variables|/Game/Blueprints/Weapons/Weapon.Weapon_C|GetRightHandHold _returnvalue_6))
  (bind _returnvalue_10 (Math|Float|Sign(Float) _x))
  (bind _returnvalue_11 (Components|GetChildComponent _output 0))
  (bind (_x_2 _y _z) (Math|Vector|BreakVector _righthandhold))
  (bind (_x_3 _y_2 _z_2) (Math|Vector|BreakVector _lefthandhold))
  (bind _returnvalue_12 (Components|GetChildComponent _output_2 0))
  (bind _aspaper_sprite_component (Utilities|Casting|CastToPaperSpriteComponent _returnvalue_12))
  (bind _aspaper_sprite_component_2 (Utilities|Casting|CastToPaperSpriteComponent _returnvalue_11))
  (bind _returnvalue_13 (* _returnvalue_10 9e+01))
  (bind _returnvalue_14 (+ _returnvalue_13 9e+01))
  ;[1 1 1] Comment
  (Variables|Default|SetRightShoulderLoc (+ (Variables|/Game/Blueprints/Entities/Entity.Entity_C|GetRightShoulderLoc (.AsEntity (Utilities|Casting|CastToEntity (Components|GetOwner)))) (* (Math|Float|Sign(Float) (.X (Math|Vector|BreakVector (Variables|/Game/Blueprints/Entities/Entity.Entity_C|GetPointDirection (.AsEntity (Utilities|Casting|CastToEntity (Components|GetOwner))))))) "0.000000,2.000000,0.000000")))
  ;[1 1 1] Comment
  (Variables|Default|SetRightHandLoc (+ (Variables|/Script/Engine.SceneComponent|GetRelativeLocation _aspaper_sprite_component_2) (Math|Vector|RotateVector (Math|Vector|MakeVector (* (* (Math|Float|Sign(Float) (.X (Math|Vector|BreakVector (Variables|/Game/Blueprints/Entities/Entity.Entity_C|GetPointDirection (.AsEntity (Utilities|Casting|CastToEntity (Components|GetOwner))))))) -1.0) _x_2) _y _z) (Variables|/Script/Engine.SceneComponent|GetRelativeRotation _aspaper_sprite_component_2)) (* (Math|Float|Sign(Float) (.X (Math|Vector|BreakVector (Variables|/Game/Blueprints/Entities/Entity.Entity_C|GetPointDirection (.AsEntity (Utilities|Casting|CastToEntity (Components|GetOwner))))))) "0.000000,1.000000,0.000000") "0.000000,2.500000,0.000000"))
  ;[1 1 1] Comment
  (Variables|Default|SetRightElbowLoc (+ (Math|Vector|MakeVector (+ (.X (Math|Vector|BreakVector (* (Math|Float|Sign(Float) (.X (Math|Vector|BreakVector (Variables|/Game/Blueprints/Entities/Entity.Entity_C|GetPointDirection (.AsEntity (Utilities|Casting|CastToEntity (Components|GetOwner))))))) (* (Math|Vector|Normalize (Math|Vector|RotateVector (- (Variables|Default|GetRightShoulderLoc) (Variables|Default|GetRightHandLoc)) "90.000000,0.000000,0.000000")) (Math|Float|Sqrt (- (Math|Float|Square (Variables|Default|GetArmLength)) (Math|Float|Square (/ (Math|Vector|Distance(Vector) (Variables|Default|GetRightShoulderLoc) (Variables|Default|GetRightHandLoc)) 2.0)))))))) (.X (Math|Vector|BreakVector (/ (+ (Variables|Default|GetRightShoulderLoc) (Variables|Default|GetRightHandLoc)) 2.0)))) (.Y (Math|Vector|BreakVector (/ (+ (Variables|Default|GetRightShoulderLoc) (Variables|Default|GetRightHandLoc)) 2.0))) (+ (.Z (Math|Vector|BreakVector (/ (+ (Variables|Default|GetRightShoulderLoc) (Variables|Default|GetRightHandLoc)) 2.0))) (.Z (Math|Vector|BreakVector (* (Math|Float|Sign(Float) (.X (Math|Vector|BreakVector (Variables|/Game/Blueprints/Entities/Entity.Entity_C|GetPointDirection (.AsEntity (Utilities|Casting|CastToEntity (Components|GetOwner))))))) (* (Math|Vector|Normalize (Math|Vector|RotateVector (- (Variables|Default|GetRightShoulderLoc) (Variables|Default|GetRightHandLoc)) "90.000000,0.000000,0.000000")) (Math|Float|Sqrt (- (Math|Float|Square (Variables|Default|GetArmLength)) (Math|Float|Square (/ (Math|Vector|Distance(Vector) (Variables|Default|GetRightShoulderLoc) (Variables|Default|GetRightHandLoc)) 2.0)))))))))) (* (Math|Float|Sign(Float) (.X (Math|Vector|BreakVector (Variables|/Game/Blueprints/Entities/Entity.Entity_C|GetPointDirection (.AsEntity (Utilities|Casting|CastToEntity (Components|GetOwner))))))) "0.000000,1.000000,0.000000")))
  ;[1 1 1] Rotate Sprites
  (Transformation|SetRelativeRotation (Variables|/Script/Paper2D.PaperCharacter|GetSprite (.AsEntity (Utilities|Casting|CastToEntity (Components|GetOwner)))) (* (Math|Rotator|MakeRotator 0.0 0.0 (+ (* _returnvalue_10 9e+01) 9e+01)) _returnvalue_10) false false)
  ;;[1 1 1] Get Weapon Sprite
  (for _array_element (Actor|GetComponentsbyTag (.AsEntity (Utilities|Casting|CastToEntity (Components|GetOwner))) "/Script/Engine.SpringArmComponent" "hand")
    (Transformation|SetRelativeRotation (.AsPaper%20Sprite%20Component (Utilities|Casting|CastToPaperSpriteComponent (Components|GetChildComponent _array_element 0))) (Math|Rotator|MakeRotator (+ _returnvalue_14 (.Roll (Math|Rotator|BreakRotator (Variables|/Script/Engine.SceneComponent|GetRelativeRotation (.AsPaper%20Sprite%20Component (Utilities|Casting|CastToPaperSpriteComponent (Components|GetChildComponent _array_element 0))))))) (+ (.Pitch (Math|Rotator|BreakRotator (Variables|/Script/Engine.SceneComponent|GetRelativeRotation (.AsPaper%20Sprite%20Component (Utilities|Casting|CastToPaperSpriteComponent (Components|GetChildComponent _array_element 0)))))) _returnvalue_14) (.Yaw (Math|Rotator|BreakRotator (Variables|/Script/Engine.SceneComponent|GetRelativeRotation (.AsPaper%20Sprite%20Component (Utilities|Casting|CastToPaperSpriteComponent (Components|GetChildComponent _array_element 0))))))) false false))
  ;[1 1 1] Set Bicep
  (Variables|Default|SetRightBicepLoc (+ (/ (+ (Variables|Default|GetRightElbowLoc) (Variables|Default|GetRightShoulderLoc)) 2.0) (* (Math|Float|Sign(Float) (.X (Math|Vector|BreakVector (Variables|/Game/Blueprints/Entities/Entity.Entity_C|GetPointDirection (.AsEntity (Utilities|Casting|CastToEntity (Components|GetOwner))))))) "0.000000,0.500000,0.000000")))
  (Transformation|SetRelativeRotation (Variables|Default|GetRightBicepSprite) (Math|Rotator|MakeRotator 0.0 (Class|KismetMathLibrary|DegAtan2 (.Z (Math|Vector|BreakVector (Math|Vector|Normalize (- (Variables|Default|GetRightElbowLoc) (Variables|Default|GetRightShoulderLoc))))) (.X (Math|Vector|BreakVector (Math|Vector|Normalize (- (Variables|Default|GetRightElbowLoc) (Variables|Default|GetRightShoulderLoc)))))) 0.0) false false)
  ;[1 1 1] Set Forearm
  (Variables|Default|SetRightForearmLoc (+ (/ (+ (Variables|Default|GetRightElbowLoc) (Variables|Default|GetRightHandLoc)) 2.0) (* (Math|Float|Sign(Float) (.X (Math|Vector|BreakVector (Variables|/Game/Blueprints/Entities/Entity.Entity_C|GetPointDirection (.AsEntity (Utilities|Casting|CastToEntity (Components|GetOwner))))))) "0.000000,1.000000,0.000000") "0.000000,0.500000,0.000000"))
  (Transformation|SetRelativeRotation (Variables|Default|GetRightForearmSprite) (Math|Rotator|MakeRotator 0.0 (Class|KismetMathLibrary|DegAtan2 (.Z (Math|Vector|BreakVector (Math|Vector|Normalize (- (Variables|Default|GetRightElbowLoc) (Variables|Default|GetRightHandLoc))))) (.X (Math|Vector|BreakVector (Math|Vector|Normalize (- (Variables|Default|GetRightElbowLoc) (Variables|Default|GetRightHandLoc)))))) 0.0) false false)
  (if (not (Variables|/Game/Blueprints/Weapons/Weapon.Weapon_C|GetOneHanded (Actor|GetComponentbyClass (.AsEntity (Utilities|Casting|CastToEntity (Components|GetOwner))) "/Game/Blueprints/Weapons/Weapon.Weapon_C")))
    ;[1 1 1] Comment
    (Variables|Default|SetLeftShoulderLoc (+ (Variables|/Game/Blueprints/Entities/Entity.Entity_C|GetLeftShoulderLoc (.AsEntity (Utilities|Casting|CastToEntity (Components|GetOwner)))) (* (Math|Float|Sign(Float) (.X (Math|Vector|BreakVector (Variables|/Game/Blueprints/Entities/Entity.Entity_C|GetPointDirection (.AsEntity (Utilities|Casting|CastToEntity (Components|GetOwner))))))) "0.000000,-0.100000,0.000000")))
    ;[1 1 1] Comment
    (Variables|Default|SetLeftHandLoc (+ (Variables|/Script/Engine.SceneComponent|GetRelativeLocation _aspaper_sprite_component) (Math|Vector|RotateVector (Math|Vector|MakeVector _x_3 _y_2 _z_2) (Variables|/Script/Engine.SceneComponent|GetRelativeRotation _aspaper_sprite_component)) "0.000000,2.000000,0.000000" "0.000000,1.000000,0.000000"))
    ;[1 1 1] Comment
    (Variables|Default|SetLeftElbowLoc (+ (Math|Vector|MakeVector (+ (.X (Math|Vector|BreakVector (* (Math|Float|Sign(Float) (.X (Math|Vector|BreakVector (Variables|/Game/Blueprints/Entities/Entity.Entity_C|GetPointDirection (.AsEntity (Utilities|Casting|CastToEntity (Components|GetOwner))))))) (* (Math|Vector|Normalize (Math|Vector|RotateVector (- (Variables|Default|GetLeftShoulderLoc) (Variables|Default|GetLeftHandLoc)) "90.000000,0.000000,0.000000")) (Math|Float|Sqrt (- (Math|Float|Square (Variables|Default|GetArmLength)) (Math|Float|Square (/ (Math|Vector|Distance(Vector) (Variables|Default|GetLeftShoulderLoc) (Variables|Default|GetLeftHandLoc)) 2.0)))))))) (.X (Math|Vector|BreakVector (/ (+ (Variables|Default|GetLeftShoulderLoc) (Variables|Default|GetLeftHandLoc)) 2.0)))) (.Y (Math|Vector|BreakVector (/ (+ (Variables|Default|GetLeftShoulderLoc) (Variables|Default|GetLeftHandLoc)) 2.0))) (+ (.Z (Math|Vector|BreakVector (/ (+ (Variables|Default|GetLeftShoulderLoc) (Variables|Default|GetLeftHandLoc)) 2.0))) (.Z (Math|Vector|BreakVector (* (Math|Float|Sign(Float) (.X (Math|Vector|BreakVector (Variables|/Game/Blueprints/Entities/Entity.Entity_C|GetPointDirection (.AsEntity (Utilities|Casting|CastToEntity (Components|GetOwner))))))) (* (Math|Vector|Normalize (Math|Vector|RotateVector (- (Variables|Default|GetLeftShoulderLoc) (Variables|Default|GetLeftHandLoc)) "90.000000,0.000000,0.000000")) (Math|Float|Sqrt (- (Math|Float|Square (Variables|Default|GetArmLength)) (Math|Float|Square (/ (Math|Vector|Distance(Vector) (Variables|Default|GetLeftShoulderLoc) (Variables|Default|GetLeftHandLoc)) 2.0)))))))))) (* (Math|Float|Sign(Float) (.X (Math|Vector|BreakVector (Variables|/Game/Blueprints/Entities/Entity.Entity_C|GetPointDirection (.AsEntity (Utilities|Casting|CastToEntity (Components|GetOwner))))))) "0.000000,-1.000000,0.000000")))
    ;[1 1 1] Set Bicep
    (Variables|Default|SetLeftBicepLoc (+ (/ (+ (Variables|Default|GetLeftElbowLoc) (Variables|Default|GetLeftShoulderLoc)) 2.0) (* (Math|Float|Sign(Float) (.X (Math|Vector|BreakVector (Variables|/Game/Blueprints/Entities/Entity.Entity_C|GetPointDirection (.AsEntity (Utilities|Casting|CastToEntity (Components|GetOwner))))))) "0.000000,-0.500000,0.000000")))
    (Transformation|SetRelativeRotation (Variables|Default|GetLeftBicepSprite) (Math|Rotator|MakeRotator 0.0 (Class|KismetMathLibrary|DegAtan2 (.Z (Math|Vector|BreakVector (Math|Vector|Normalize (- (Variables|Default|GetLeftElbowLoc) (Variables|Default|GetLeftShoulderLoc))))) (.X (Math|Vector|BreakVector (Math|Vector|Normalize (- (Variables|Default|GetLeftElbowLoc) (Variables|Default|GetLeftShoulderLoc)))))) 0.0) false false)
    ;[1 1 1] Set Forearm
    (Variables|Default|SetLeftForearmLoc (+ (/ (+ (Variables|Default|GetLeftElbowLoc) (Variables|Default|GetLeftHandLoc)) 2.0) (* (Math|Float|Sign(Float) (.X (Math|Vector|BreakVector (Variables|/Game/Blueprints/Entities/Entity.Entity_C|GetPointDirection (.AsEntity (Utilities|Casting|CastToEntity (Components|GetOwner))))))) "0.000000,-1.000000,0.000000")))
    (Transformation|SetRelativeRotation (Variables|Default|GetLeftForearmSprite) (Math|Rotator|MakeRotator 0.0 (Class|KismetMathLibrary|DegAtan2 (.Z (Math|Vector|BreakVector (Math|Vector|Normalize (- (Variables|Default|GetLeftElbowLoc) (Variables|Default|GetLeftHandLoc))))) (.X (Math|Vector|BreakVector (Math|Vector|Normalize (- (Variables|Default|GetLeftElbowLoc) (Variables|Default|GetLeftHandLoc)))))) 0.0) false false)
    ;[1 1 1] Apply Location
    (Transformation|SetRelativeLocation (Variables|Default|GetRightShoulderSprite) (Variables|Default|GetRightShoulderLoc) false false)
    (Transformation|SetRelativeLocation (Variables|Default|GetRightBicepSprite) (Variables|Default|GetRightBicepLoc) false false)
    (Transformation|SetRelativeLocation (Variables|Default|GetRightElbowSprite) (Variables|Default|GetRightElbowLoc) false false)
    (Transformation|SetRelativeLocation (Variables|Default|GetRightForearmSprite) (Variables|Default|GetRightForearmLoc) false false)
    (Transformation|SetRelativeLocation (Variables|Default|GetRightHandSprite) (Variables|Default|GetRightHandLoc) false false)
    (if (not (Variables|/Game/Blueprints/Weapons/Weapon.Weapon_C|GetOneHanded (Actor|GetComponentbyClass (.AsEntity (Utilities|Casting|CastToEntity (Components|GetOwner))) "/Game/Blueprints/Weapons/Weapon.Weapon_C")))
      (Transformation|SetRelativeLocation (Variables|Default|GetLeftShoulderSprite) (Variables|Default|GetLeftShoulderLoc) false false)
      (Transformation|SetRelativeLocation (Variables|Default|GetLeftBicepSprite) (Variables|Default|GetLeftBicepLoc) false false)
      (Transformation|SetRelativeLocation (Variables|Default|GetLeftElbowSprite) (Variables|Default|GetLeftElbowLoc) false false)
      (Transformation|SetRelativeLocation (Variables|Default|GetLeftForearmSprite) (Variables|Default|GetLeftForearmLoc) false false)
      (Transformation|SetRelativeLocation (Variables|Default|GetLeftHandSprite) (Variables|Default|GetLeftHandLoc) false false))))