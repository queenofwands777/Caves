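; MenuGhost is a player-controlled character that flies in the XZ plane, aims at the mouse and fires one of ten switchable weapons.
; Axis inputs feed a swept offset move on Tick, which also orbits the held weapon toward the cursor and pushes health and ammo to the HUD.
; GetHit subtracts health, spawns blood splatter from bullet parameters and ends the game at zero health.
; Interact pickup is an empty stub.
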(event EventBeginPlay
  ;[1 1 1] initialize hud values
  (bind _foundwidgets (Widget|GetAllWidgetsOfClass "/Game/Blueprints/UI/HUD.HUD_C" true))
  (for _array_element _foundwidgets
    (Variables|/Game/Blueprints/UI/HUD.HUD_C|SetPlayerHealth _array_element (Variables|Default|GetHealth))
    (Variables|/Game/Blueprints/UI/HUD.HUD_C|SetPlayerAmmo _array_element (Variables|Default|GetAmmo))))

(event EventTick
  (params (DeltaSeconds :type Float%20%28single-precision%29))
  (bind _returnvalue (Actor|GetComponentbyClass "/Game/Blueprints/Weapons/Weapon.Weapon_C"))
  (bind _hand (Variables|Default|Gethand))
  (bind _returnvalue_2 (Components|GetChildComponent _hand 0))
  (bind _locationoffset (Variables|/Game/Blueprints/Weapons/Weapon.Weapon_C|GetLocationOffset _returnvalue))
  ;[1 1 1] Player Movement
  (if (Variables|Default|GetAlive)
    (CallFunction|CustomMove (Variables|Default|GetUpDown) (Variables|Default|GetLeftRight) DeltaSeconds)
    (Variables|Default|SetUpDown 0.0)
    (Variables|Default|SetLeftRight 0.0)
    ;[1 1 1] Weapon rotation
    (bind _returnvalue_3 (Class|WidgetLayoutLibrary|GetMousePositiononViewport))
    (Transformation|SetRelativeRotation _returnvalue_2 (Math|Rotator|MakeRotator (+ (* (Math|Float|Sign(Float) (.X (Math|Vector|BreakVector (Math|Vector|Normalize (Math|Conversions|ToVector(Vector2D) (- _returnvalue_3 (Class|SlateBlueprintLibrary|ScreentoViewport (.ScreenPosition (Class|GameplayStatics|ProjectWorldtoScreen (Game|GetPlayerController 0) (Transformation|GetActorLocation) false))))))))) 9e+01) 9e+01) (+ (+ (* (Math|Float|Sign(Float) (.X (Math|Vector|BreakVector (Math|Vector|Normalize (Math|Conversions|ToVector(Vector2D) (- _returnvalue_3 (Class|SlateBlueprintLibrary|ScreentoViewport (.ScreenPosition (Class|GameplayStatics|ProjectWorldtoScreen (Game|GetPlayerController 0) (Transformation|GetActorLocation) false))))))))) 9e+01) 9e+01) (+ (* (Class|KismetMathLibrary|DegAsin (Math|Vector|DotProduct (Math|Vector|MakeVector (.X (Math|Vector|BreakVector (Math|Vector|Normalize (Math|Conversions|ToVector(Vector2D) (- _returnvalue_3 (Class|SlateBlueprintLibrary|ScreentoViewport (.ScreenPosition (Class|GameplayStatics|ProjectWorldtoScreen (Game|GetPlayerController 0) (Transformation|GetActorLocation) false)))))))) 0.0 (.Y (Math|Vector|BreakVector (Math|Vector|Normalize (Math|Conversions|ToVector(Vector2D) (- _returnvalue_3 (Class|SlateBlueprintLibrary|ScreentoViewport (.ScreenPosition (Class|GameplayStatics|ProjectWorldtoScreen (Game|GetPlayerController 0) (Transformation|GetActorLocation) false))))))))) "1.000000,0.000000,0.000000")) (Math|Float|Sign(Float) (.Y (Math|Vector|BreakVector (Math|Vector|Normalize (Math|Conversions|ToVector(Vector2D) (- _returnvalue_3 (Class|SlateBlueprintLibrary|ScreentoViewport (.ScreenPosition (Class|GameplayStatics|ProjectWorldtoScreen (Game|GetPlayerController 0) (Transformation|GetActorLocation) false)))))))))) (+ (* (Math|Float|Sign(Float) (.Y (Math|Vector|BreakVector (Math|Vector|Normalize (Math|Conversions|ToVector(Vector2D) (- _returnvalue_3 (Class|SlateBlueprintLibrary|ScreentoViewport (.ScreenPosition (Class|GameplayStatics|ProjectWorldtoScreen (Game|GetPlayerController 0) (Transformation|GetActorLocation) false))))))))) 9e+01) 9e+01))) 0.0) false false)
    (Transformation|SetRelativeLocation _returnvalue_2 (Math|Vector|MakeVector (+ 0.0 (* (.X (Math|Vector|BreakVector (Math|Vector|MakeVector (.X (Math|Vector|BreakVector (Math|Vector|Normalize (Math|Conversions|ToVector(Vector2D) (- _returnvalue_3 (Class|SlateBlueprintLibrary|ScreentoViewport (.ScreenPosition (Class|GameplayStatics|ProjectWorldtoScreen (Game|GetPlayerController 0) (Transformation|GetActorLocation) false)))))))) 0.0 (.Y (Math|Vector|BreakVector (Math|Vector|Normalize (Math|Conversions|ToVector(Vector2D) (- _returnvalue_3 (Class|SlateBlueprintLibrary|ScreentoViewport (.ScreenPosition (Class|GameplayStatics|ProjectWorldtoScreen (Game|GetPlayerController 0) (Transformation|GetActorLocation) false))))))))))) _locationoffset)) 1.0 (* (+ 0.0 (* (.Z (Math|Vector|BreakVector (Math|Vector|MakeVector (.X (Math|Vector|BreakVector (Math|Vector|Normalize (Math|Conversions|ToVector(Vector2D) (- _returnvalue_3 (Class|SlateBlueprintLibrary|ScreentoViewport (.ScreenPosition (Class|GameplayStatics|ProjectWorldtoScreen (Game|GetPlayerController 0) (Transformation|GetActorLocation) false)))))))) 0.0 (.Y (Math|Vector|BreakVector (Math|Vector|Normalize (Math|Conversions|ToVector(Vector2D) (- _returnvalue_3 (Class|SlateBlueprintLibrary|ScreentoViewport (.ScreenPosition (Class|GameplayStatics|ProjectWorldtoScreen (Game|GetPlayerController 0) (Transformation|GetActorLocation) false))))))))))) _locationoffset)) -1.0)) false false)
    ;[1 1 1] Update HUD
    (bind _foundwidgets (Widget|GetAllWidgetsOfClass "/Game/Blueprints/UI/HUD.HUD_C" true))
    (for _array_element _foundwidgets
      (Variables|/Game/Blueprints/UI/HUD.HUD_C|SetPlayerHealth _array_element (Variables|Default|GetHealth))
      (Variables|/Game/Blueprints/UI/HUD.HUD_C|SetPlayerAmmo _array_element (Variables|Default|GetAmmo)))))

(event Input|ActionEvents|InputActionFire
  (params (Key :type Key%20Structure :default "None"))
  (:Pressed
    (if (Variables|Default|GetAlive)
      ;[1 1 1] Fire Weapon
      (bind _returnvalue (Class|WidgetLayoutLibrary|GetMousePositiononViewport))
      (if (> (Variables|Default|GetAmmo) 0)
        (Default|FireWeapon (Actor|GetComponentbyClass "/Game/Blueprints/Weapons/Weapon.Weapon_C") (* (Math|Vector|Normalize (Math|Vector|MakeVector (.X (Math|Vector2D|BreakVector2D (- _returnvalue (Class|SlateBlueprintLibrary|ScreentoViewport (.ScreenPosition (Class|GameplayStatics|ProjectWorldtoScreen (Game|GetPlayerController 0) (Transformation|GetActorLocation) false)))))) 0.0 (.Y (Math|Vector2D|BreakVector2D (- _returnvalue (Class|SlateBlueprintLibrary|ScreentoViewport (.ScreenPosition (Class|GameplayStatics|ProjectWorldtoScreen (Game|GetPlayerController 0) (Transformation|GetActorLocation) false)))))))) (Math|Vector|MakeVector 1.0 0.0 -1.0)))
        (Math|Integer|DecrementInt (Variables|Default|GetAmmo))))))

(event Input|ActionEvents|InputActionInteract
  (params (Key :type Key%20Structure :default "None"))
  ;[1 1 1] Weapon pickup
  (:Pressed
    ;;[1 1 1] if overlap katana, equip
    (if true
      _)))

(event Input|AxisEvents|InputAxisUp
  (params (AxisValue :type Float%20%28single-precision%29))
  ;[1 1 1] Player Movement
  (if (Variables|Default|GetAlive)
    (Variables|Default|SetUpDown (+ AxisValue (Variables|Default|GetUpDown)))))

(event Input|AxisEvents|InputAxisLeft
  (params (AxisValue :type Float%20%28single-precision%29))
  ;[1 1 1] Player Movement
  (if (Variables|Default|GetAlive)
    (Variables|Default|SetLeftRight (+ AxisValue (Variables|Default|GetLeftRight)))))

(event Input|AxisEvents|InputAxisSwitch
  (params (AxisValue :type Float%20%28single-precision%29))
  (if (Variables|Default|GetAlive)
    ;[1 1 1] Switch Weapon
    (Components|DestroyComponent (Actor|GetComponentbyClass "/Game/Blueprints/Weapons/Weapon.Weapon_C"))
    (Components|DestroyComponent (Components|GetChildComponent (Variables|Default|Gethand) 0))
    (Variables|Default|Setweaponslot (Math|Integer|%(Integer) (+ AxisValue (Variables|Default|Getweaponslot)) 10))
    (switch int (Variables|Default|Getweaponslot)
      (:0
        (Game|AddComponentbyClass "/Game/Blueprints/Weapons/Ranged/AutoRifle.AutoRifle_C"))
      (:1
        (Game|AddComponentbyClass "/Game/Blueprints/Weapons/Ranged/BurstRifle.BurstRifle_C"))
      (:2
        (Game|AddComponentbyClass "/Game/Blueprints/Weapons/Ranged/Pistol.Pistol_C"))
      (:3
        (Game|AddComponentbyClass "/Game/Blueprints/Weapons/Ranged/Uzi.Uzi_C"))
      (:4
        (Game|AddComponentbyClass "/Game/Blueprints/Weapons/Ranged/GrenadeLauncher.GrenadeLauncher_C"))
      (:5
        (Game|AddComponentbyClass "/Game/Blueprints/Weapons/Ranged/Shotgun.Shotgun_C"))
      (:6
        (Game|AddComponentbyClass "/Game/Blueprints/Weapons/Melee/Katana.Katana_C"))
      (:7
        (Game|AddComponentbyClass "/Game/Blueprints/Weapons/Melee/Chainsaw.Chainsaw_C"))
      (:8
        (Game|AddComponentbyClass "/Game/Blueprints/Weapons/Melee/Hammer.Hammer_C"))
      (:9
        (Game|AddComponentbyClass "/Game/Blueprints/Weapons/Melee/Shank.Shank_C")))))

(fn ConstructionScript)

(fn CustomMove
  (params (UpDown :type Float%20%28double-precision%29) (LeftRight :type Float%20%28double-precision%29) (DeltaTime :type Float%20%28double-precision%29))
  (bind _sweephitresult (Transformation|AddActorWorldOffset (* (* (Variables|Default|GetSpeed) DeltaTime) (Math|Vector|MakeVector LeftRight 0.0 UpDown)) true))
  (if (.bBlockingHit (Collision|BreakHitResult _sweephitresult))
    (Class|NavMovementComponent|StopActiveMovement (Variables|Character|GetCharacterMovement))))

(fn GetHit
  (params (Damage :type Integer) (Bullet :type Enemy%20Bullet%20Object%20Reference))
  (bind _returnvalue (Transformation|GetActorTransform))
  (bind (_location _rotation _scale) (Math|Transform|BreakTransform _returnvalue))
  (bind (_x _y _z) (Math|Vector|BreakVector _location))
  (bind (_roll _pitch _yaw) (Math|Rotator|BreakRotator _rotation))
  (Variables|Default|SetHealth (- (Variables|Default|GetHealth) Damage))
  (bind _returnvalue_2 (Game|SpawnActorfromClass "/Script/Caves.BloodSplatter" (Math|Transform|MakeTransform (Math|Vector|MakeVector (+ 0.0 _x) 1.0 (+ _z 0.0)) (Math|Rotator|MakeRotator _roll _pitch _yaw) _scale) "Undefined" "MultiplyWithRoot" 0 0))
  (Class|BloodSplatter|InitParams _returnvalue_2 (Variables|/Game/Blueprints/Weapons/Projectiles/PlayerBullet.PlayerBullet_C|GetNumProbes Bullet) (Variables|/Game/Blueprints/Weapons/Projectiles/PlayerBullet.PlayerBullet_C|GetBloodQuantity Bullet) (Variables|/Game/Blueprints/Weapons/Projectiles/PlayerBullet.PlayerBullet_C|GetMaxAngle Bullet) (Variables|/Game/Blueprints/Weapons/Projectiles/PlayerBullet.PlayerBullet_C|GetProbeLifetime Bullet) (Variables|/Game/Blueprints/Weapons/Projectiles/PlayerBullet.PlayerBullet_C|GetProbeVariance Bullet) (Variables|/Game/Blueprints/Weapons/Projectiles/PlayerBullet.PlayerBullet_C|GetProbeSpeed Bullet) (Variables|/Game/Blueprints/Weapons/Projectiles/PlayerBullet.PlayerBullet_C|GetDirection Bullet) (Transformation|GetActorLocation))
  (Class|BloodSplatter|Splatter _returnvalue_2)
  (if (Math|Conversions|ToBoolean(Integer) (Class|KismetMathLibrary|AndIntInt (Math|Conversions|ToInteger(Boolean) (<= (Variables|Default|GetHealth) 0)) (Math|Conversions|ToInteger(Boolean) (Variables|Default|GetAlive))))
    (bind _asgame (Utilities|Casting|CastToGame (Game|GetGameInstance)))
    (Variables|Default|SetAlive false)
    (Default|EndGame _asgame)))