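; Entity is a base-style actor for damageable game objects with health, hit reactions and knockback.
; GetHit subtracts damage, then spawns a BloodSplatter at a fixed Y plane, configured from the hitting bullet's spray parameters and direction.
; When health runs out it marks itself dead, spawns a Remains actor and destroys itself.
; KnockBack applies a velocity-change impulse to the capsule.
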(event EventBeginPlay)

(event Collision|EventActorBeginOverlap
  (params (OtherActor :type Actor%20Object%20Reference)))

(event EventTick
  (params (DeltaSeconds :type Float%20%28single-precision%29)))

(fn ConstructionScript)

(fn GetHit
  (params (Damage :type Integer) (Bullet :type Projectile%20Object%20Reference))
  (bind _returnvalue (Transformation|GetActorTransform))
  (bind (_location _rotation _scale) (Math|Transform|BreakTransform _returnvalue))
  (bind (_x _y _z) (Math|Vector|BreakVector _location))
  (bind (_roll _pitch _yaw) (Math|Rotator|BreakRotator _rotation))
  (Variables|Default|SetHealth (- (Variables|Default|GetHealth) Damage))
  (bind _returnvalue_2 (Game|SpawnActorfromClass "/Script/Caves.BloodSplatter" (Math|Transform|MakeTransform (Math|Vector|MakeVector (+ 0.0 _x) 1.0 (+ _z 0.0)) (Math|Rotator|MakeRotator _roll _pitch _yaw) _scale) "Undefined" "MultiplyWithRoot" 0 0))
  (Class|BloodSplatter|InitParams _returnvalue_2 (Variables|/Game/Blueprints/Weapons/Projectiles/PlayerBullet.PlayerBullet_C|GetNumProbes Bullet) (Variables|/Game/Blueprints/Weapons/Projectiles/PlayerBullet.PlayerBullet_C|GetBloodQuantity Bullet) (Variables|/Game/Blueprints/Weapons/Projectiles/PlayerBullet.PlayerBullet_C|GetMaxAngle Bullet) (Variables|/Game/Blueprints/Weapons/Projectiles/PlayerBullet.PlayerBullet_C|GetProbeLifetime Bullet) 3 (Variables|/Game/Blueprints/Weapons/Projectiles/PlayerBullet.PlayerBullet_C|GetProbeVariance Bullet) (Variables|/Game/Blueprints/Weapons/Projectiles/PlayerBullet.PlayerBullet_C|GetProbeSpeed Bullet) (Variables|/Game/Blueprints/Weapons/Projectiles/Projectile.Projectile_C|GetDirection Bullet) (Transformation|GetActorLocation))
  (Class|BloodSplatter|Splatter _returnvalue_2)
  (if (<= (Variables|Default|GetHealth) 0)
    (Variables|Default|SetAlive false)
    (Game|SpawnActorfromClass "/Script/Caves.Remains" (Transformation|GetActorTransform) "Undefined" "MultiplyWithRoot" 0 0)
    (Actor|DestroyActor)))

(fn KnockBack
  (params (Direction :type Vector) (Magnitude :type Float%20%28double-precision%29))
  (Physics|AddImpulse (Variables|Collision|GetCapsuleComponent) (* Direction Magnitude) "None" true))