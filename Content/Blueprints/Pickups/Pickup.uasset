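; A base 2D pickup actor that highlights when the player is in range and can be collected manually or automatically.
; Overlap events on the Pickup component swap the Paper sprite between normal and glowing materials and set an InRange flag.
; While in range and unlocked, Tick polls the player's Interacting flag or AutoPickUp, then plays a sound and calls Interact.
; Interact is empty here, apparently left for child Blueprints to override.
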(event OnComponentBeginOverlap(pickup)
  (params (OverlappedComponent :type Primitive%20Component%20Object%20Reference) (OtherActor :type Actor%20Object%20Reference) (OtherComp :type Primitive%20Component%20Object%20Reference) (OtherBodyIndex :type Integer) (bFromSweep :type Boolean) (SweepResult :type Hit%20Result%20Structure%20%28by%20ref%29))
  (Utilities|Casting|CastToplayer OtherActor)
  (Rendering|Material|SetMaterial (Variables|Default|GetPaperSprite) 0 "/Game/Assets/Materials/GlowingPickupMaterial.GlowingPickupMaterial")
  (Variables|Default|SetInRange true))

(event OnComponentEndOverlap(pickup)
  (params (OverlappedComponent :type Primitive%20Component%20Object%20Reference) (OtherActor :type Actor%20Object%20Reference) (OtherComp :type Primitive%20Component%20Object%20Reference) (OtherBodyIndex :type Integer))
  (Utilities|Casting|CastToplayer OtherActor)
  (Rendering|Material|SetMaterial (Variables|Default|GetPaperSprite) 0 "/Game/Assets/Materials/PickupMaterial.PickupMaterial")
  (Variables|Default|SetInRange false))

(event EventBeginPlay
  (Rendering|Material|SetMaterial (Variables|Default|GetPaperSprite) 0 "/Game/Assets/Materials/PickupMaterial.PickupMaterial"))

(event Collision|EventActorBeginOverlap
  (params (OtherActor :type Actor%20Object%20Reference)))

(event EventTick
  (params (DeltaSeconds :type Float%20%28single-precision%29))
  (if (Variables|Default|GetInRange)
    (bind _returnvalue (Actor|GetActorOfClass "/Game/Blueprints/Entities/player.player_C"))
    (if (not (Variables|Default|GetLocked))
      (if (Variables|/Game/Blueprints/Entities/player.player_C|GetInteracting _returnvalue)
        (Audio|PlaySoundatLocation (Variables|Default|GetPickupSound) (Transformation|GetActorLocation self) "0, 0, 0" 1.0 1.0 0.0 0 0 0 0)
        (CallFunction|Interact _returnvalue)
        (elif (Variables|Default|GetAutoPickUp)
          (Audio|PlaySoundatLocation (Variables|Default|GetPickupSound) (Transformation|GetActorLocation self) "0, 0, 0" 1.0 1.0 0.0 0 0 0 0)
          (CallFunction|Interact _returnvalue))))))

(fn ConstructionScript)

(fn Interact
  (params (Player :type Player%20Object%20Reference)))