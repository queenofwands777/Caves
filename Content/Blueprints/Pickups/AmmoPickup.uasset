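; Ammo pickup actor that grants ammunition to a player who interacts with it.
; Its Interact function checks the player's Interacting flag, adds a fixed amount to the player's Ammo, then destroys the pickup.
; BeginPlay, Tick and the construction script hold no logic beyond parent calls.
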(event EventBeginPlay
  (|CallParentFunction) ; This node is disabled and will not be called.\nDrag off pins to build functionality.
)

(event EventTick
  (params (DeltaSeconds :type Float%20%28single-precision%29))
  (|CallParentFunction DeltaSeconds) ; This node is disabled and will not be called.\nDrag off pins to build functionality.
)

(fn ConstructionScript
  (|CallParentFunction))

(fn Interact
  (params (Player :type Player%20Object%20Reference))
  (if (Variables|/Game/Blueprints/Entities/player.player_C|GetInteracting Player)
    (Variables|/Game/Blueprints/Entities/player.player_C|SetAmmo Player (+ 50 (Variables|/Game/Blueprints/Entities/player.player_C|GetAmmo Player)))
    (Actor|DestroyActor)))