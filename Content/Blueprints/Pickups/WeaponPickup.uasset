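; WeaponPickup is a pickup actor that switches the player's weapon when interacted with.
; Interact runs only while the player's Interacting flag is set, clears it, calls SwitchWeapon with the weapon class and the pickup's own class, then destroys itself.
; GetWeaponClass returns nothing here, so it serves as a hook for child pickups to supply their weapon.
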(event EventBeginPlay
  (|CallParentFunction) ; This node is disabled and will not be called.\nDrag off pins to build functionality.
)

(event EventTick
  (params (DeltaSeconds :type Float%20%28single-precision%29))
  (|CallParentFunction DeltaSeconds) ; This node is disabled and will not be called.\nDrag off pins to build functionality.
)

(fn ConstructionScript
  (|CallParentFunction))

(fn GetWeaponClass
  (return 0))

(fn Interact
  (params (Player :type Player%20Object%20Reference))
  (if (Variables|/Game/Blueprints/Entities/player.player_C|GetInteracting Player)
    (Variables|/Game/Blueprints/Entities/player.player_C|SetInteracting Player false)
    (bind _newparam (CallFunction|GetWeaponClass))
    (Default|SwitchWeapon Player _newparam (Utilities|GetClass self))
    (Actor|DestroyActor)))