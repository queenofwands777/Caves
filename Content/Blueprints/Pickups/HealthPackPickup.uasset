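; Health pack pickup that restores a fixed amount of a player's health and is then consumed.
; Its Interact function acts only while the passed player's Interacting flag is set, capping the new health at the maximum stored in the GameVar game instance before destroying the actor.
; The event graph holds only disabled default events, so the pickup has no overlap or tick logic of its own.
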(event EventBeginPlay
  (|CallParentFunction) ; This node is disabled and will not be called.\nDrag off pins to build functionality.
)

(event Collision|EventActorBeginOverlap
  (params (OtherActor :type Actor%20Object%20Reference))
  (|CallParentFunction OtherActor) ; This node is disabled and will not be called.\nDrag off pins to build functionality.
)

(event EventTick
  (params (DeltaSeconds :type Float%20%28single-precision%29))
  (|CallParentFunction DeltaSeconds) ; This node is disabled and will not be called.\nDrag off pins to build functionality.
)

(fn ConstructionScript
  (|CallParentFunction))

(fn Interact
  (params (Player :type Player%20Object%20Reference))
  (if (Variables|/Game/Blueprints/Entities/player.player_C|GetInteracting Player)
    (bind _asgame_var (Utilities|Casting|CastToGameVar (Game|GetGameInstance)))
    (Variables|/Game/Blueprints/Entities/Entity.Entity_C|SetHealth Player (Math|Integer|Min(Integer) (+ 20 (Variables|/Game/Blueprints/Entities/Entity.Entity_C|GetHealth Player)) (Variables|/Game/Blueprints/Engine/GameVar.GameVar_C|GetPlayerMaxHealth _asgame_var)))
    (Actor|DestroyActor)))