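; Chest is an interactable loot pickup that releases items and is consumed when a player interacts with it.
; Interact calls OpenChest, then destroys the chest actor.
; OpenChest spawns an ammo pickup and a random entry from the Weapons class array, each at a random X and Z offset around the chest's location.
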(event EventBeginPlay
  (|CallParentFunction) ; This node is disabled and will not be called.\nDrag off pins to build functionality.
)

(event EventTick
  (params (DeltaSeconds :type Float%20%28single-precision%29))
  (|CallParentFunction DeltaSeconds) ; This node is disabled and will not be called.\nDrag off pins to build functionality.
)

(fn ConstructionScript
  (|CallParentFunction))

(fn OpenChest
  (params (Player :type Player%20Object%20Reference))
  (bind _returnvalue (Transformation|GetActorLocation))
  (bind _returnvalue_2 (Transformation|GetActorLocation))
  (bind _weapons (Variables|Default|GetWeapons))
  (bind (_x _y _z) (Math|Vector|BreakVector _returnvalue))
  (bind (_x_2 _y_2 _z_2) (Math|Vector|BreakVector _returnvalue_2))
  (Game|SpawnActorfromClass "/Game/Blueprints/Pickups/GeneralPickups/AmmoPickup.AmmoPickup_C" (Math|Transform|MakeTransform (Math|Vector|MakeVector (+ _x (Math|Random|RandomFloatinRange -5e+01 5e+01)) _y (+ (Math|Random|RandomFloatinRange -5e+01 5e+01) _z))) "Undefined" "MultiplyWithRoot" 0 0)
  (Game|SpawnActorfromClass (Utilities|Array|Get(acopy) _weapons (Math|Random|RandomInteger (Utilities|Array|Length _weapons))) (Math|Transform|MakeTransform (Math|Vector|MakeVector (+ _x_2 (Math|Random|RandomFloatinRange -5e+01 5e+01)) (+ _y_2 0.1) (+ (Math|Random|RandomFloatinRange -5e+01 5e+01) _z_2))) "Undefined" "MultiplyWithRoot" 0 0))

(fn Interact
  (params (Player :type Player%20Object%20Reference))
  (CallFunction|OpenChest Player)
  (Actor|DestroyActor))