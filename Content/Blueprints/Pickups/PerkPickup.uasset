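; Base perk pickup actor that grants a perk component to the player who interacts with it.
; Interact adds the class from GetPerk, which is empty here and presumably overridden by children, then puts the pickup's sprite on every HUD widget as a perk icon.
; It removes its own class from the game instance's PerksRemaining pool, unless only one entry or fewer is left, then destroys itself.
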(event EventBeginPlay
  (|CallParentFunction) ; This node is disabled and will not be called.\nDrag off pins to build functionality.
)

(event Collision|EventActorBeginOverlap
  (params (OtherActor :type Actor%20Object%20Reference))
  (|CallParentFunction OtherActor) ; This node is disabled and will not be called.\nDrag off pins to build functionality.
)

(event EventTick
  (params (DeltaSeconds :type Float%20%28single-precision%29))
  (|CallParentFunction DeltaSeconds) ; This node is disabled and will not be called.\nDrag off pins to build functionality.
)

(fn ConstructionScript
  (|CallParentFunction))

(fn Interact
  (params (Player :type Player%20Object%20Reference))
  (if (Variables|/Game/Blueprints/Entities/player.player_C|GetInteracting Player)
    (bind _newparam (CallFunction|GetPerk))
    (Game|AddComponentbyClass Player _newparam)
    (bind _foundwidgets (Widget|GetAllWidgetsOfClass "/Game/Blueprints/UI/HUD.HUD_C" true))
    (for _array_element _foundwidgets
      (Default|AddPerkIcon _array_element (Class|PaperSpriteBlueprintLibrary|MakeBrushfromSprite (Variables|/Script/Paper2D.PaperSpriteComponent|GetSourceSprite (Variables|Default|GetPaperSprite)) 80 16)))
    (bind _asgame_var (Utilities|Casting|CastToGameVar (Game|GetGameInstance)))
    (if (> (Utilities|Array|Length (Variables|/Game/Blueprints/Engine/GameVar.GameVar_C|GetPerksRemaining _asgame_var)) 1)
      (Utilities|Array|RemoveItem (Variables|/Game/Blueprints/Engine/GameVar.GameVar_C|GetPerksRemaining _asgame_var) (Utilities|GetClass self)))
    (Actor|DestroyActor)))

(fn GetPerk
  (return 0))