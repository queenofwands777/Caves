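; Swing is a short-lived melee attack actor with a Paper2D sprite hitbox that follows the player's movement and registers one hit.
; Each tick it applies the player's position delta and counts frames, destroying itself past its maximum lifetime.
; Overlapping WorldStatic uses up the hit; otherwise the first overlap spawns several BloodProbe actors, their direction rotated 90 degrees in the XZ plane according to IsLeft.
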(event OnComponentBeginOverlap(PaperSprite)
  (params (OverlappedComponent :type Primitive%20Component%20Object%20Reference) (OtherActor :type Actor%20Object%20Reference) (OtherComp :type Primitive%20Component%20Object%20Reference) (OtherBodyIndex :type Integer) (bFromSweep :type Boolean) (SweepResult :type Hit%20Result%20Structure%20%28by%20ref%29))
  (bind _direction (Variables|Default|GetDirection))
  (bind _direction_2 (Variables|Default|GetDirection))
  (bind (_x _y _z) (Math|Vector|BreakVector _direction))
  (bind (_x_2 _y_2 _z_2) (Math|Vector|BreakVector _direction_2))
  (if (== (Math|Conversions|ToInteger(Byte) (Collision|GetCollisionObjectType OtherComp)) (Math|Conversions|ToInteger(Byte) (Utilities|Enum|LiteralenumECollisionChannel "ECC_WorldStatic")))
    (Variables|Default|SetHitMade true)
    (elif (not (Variables|Default|GetHitMade))
      (Development|PrintString (Utilities|GetDisplayName OtherActor))
      (for _index (range 0 3)
        (if (Variables|Default|GetIsLeft)
          (Game|SpawnActorfromClass "/Game/Blueprints/BloodProbe.BloodProbe_C" (Math|Conversions|ToTransform(Vector) (+ "0.000000,-2.000000,0.000000" (Transformation|GetActorLocation))) "Undefined" "MultiplyWithRoot" 0 (Math|Vector|MakeVector (* 1.0 _z_2) _y_2 (* -1.0 _x_2)) 0)
          (else
            (Game|SpawnActorfromClass "/Game/Blueprints/BloodProbe.BloodProbe_C" (Math|Conversions|ToTransform(Vector) (+ "0.000000,-2.000000,0.000000" (Transformation|GetActorLocation))) "Undefined" "MultiplyWithRoot" 0 (Math|Vector|MakeVector (* -1.0 _z) _y (* 1.0 _x)) 0)))
        (Variables|Default|SetHitMade true)))))

(event EventBeginPlay
  (Variables|Default|Setstartloc (Transformation|GetActorLocation (Variables|Default|Getplayer)))
  (Development|PrintString (Utilities|String|ToString(Vector) (Variables|Default|GetDirection))))

(event EventTick
  (params (DeltaSeconds :type Float%20%28single-precision%29))
  (bind _player (Variables|Default|Getplayer))
  (bind _returnvalue (Transformation|GetActorLocation _player))
  (Transformation|AddActorWorldOffset (- _returnvalue (Variables|Default|Getstartloc)))
  (Variables|Default|Setstartloc _returnvalue)
  (Variables|Default|SetCurrentLifetime (+ 1.0 (Variables|Default|GetCurrentLifetime)))
  (if (> (Variables|Default|GetCurrentLifetime) (Variables|Default|GetLifetimeMax))
    (Actor|DestroyActor)))

(fn ConstructionScript)