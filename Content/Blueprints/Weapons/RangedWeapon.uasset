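; Ranged weapon Blueprint whose FireWeapon spawns projectiles at the owner's hand while selected and ammo remains.
; Spawn point follows the hand's rotated offset in the XZ plane, where multiple shots fan across Spread and single shots deviate randomly.
; The owning Entity's multipliers scale projectile damage, blood and probe settings.
; Each projectile plays a sound, consumes AmmoPerShot and receives the weapon's Aura components.
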(event EventBeginPlay
  (|CallParentFunction) ; This node is disabled and will not be called.\nDrag off pins to build functionality.
)

(fn FireWeapon
  (params (Direction :type Vector :default "0, 0, 0"))
  (bind (_x _y _z) (Math|Vector|BreakVector Direction))
  (bind _returnvalue (Components|GetOwner))
  (bind _projectileoffset (Variables|Default|GetProjectileOffset))
  (bind _spread (Variables|Default|GetSpread))
  (bind _returnvalue_2 (Actor|GetComponentsbyTag _returnvalue "/Script/Engine.SpringArmComponent" "hand"))
  (bind _returnvalue_3 (Transformation|GetActorTransform _returnvalue))
  (bind (_location _rotation _scale) (Math|Transform|BreakTransform _returnvalue_3))
  (bind _output (Utilities|Array|Get(acopy) _returnvalue_2))
  (bind _returnvalue_4 (Components|GetChildComponent _output 0))
  (bind _relativelocation (Variables|/Script/Engine.SceneComponent|GetRelativeLocation _returnvalue_4))
  (bind _relativerotation (Variables|/Script/Engine.SceneComponent|GetRelativeRotation _returnvalue_4))
  (bind _returnvalue_5 (Math|Vector|RotateVector _projectileoffset _relativerotation))
  (bind _returnvalue_6 (+ _location _relativelocation))
  (bind (_x_2 _y_2 _z_2) (Math|Vector|BreakVector _returnvalue_6))
  (bind (_x_3 _y_3 _z_3) (Math|Vector|BreakVector _returnvalue_5))
  (bind _returnvalue_7 (+ _z_2 _z_3))
  (bind _returnvalue_8 (+ _x_2 _x_3))
  (bind _returnvalue_9 (Math|Vector|MakeVector _returnvalue_8 _y_2 _returnvalue_7))
  (if (Variables|Default|GetSelected)
    (for _index (range 0 (- (Variables|Default|GetProjectilesPerShot) 1))
      (if (> (Variables|Default|GetAmmo) 0)
        (bind _asentity (Utilities|Casting|CastToEntity (Components|GetOwner)))
        (bind _returnvalue_10 (Game|SpawnActorfromClass (Variables|Default|GetProjectile) (Math|Transform|MakeTransform _returnvalue_9 _rotation _scale) "Undefined" "MultiplyWithRoot" (Components|GetOwner) (Utilities|Select :Index (Math|Conversions|ToInteger(Boolean) (== (Variables|Default|GetProjectilesPerShot) 1)) :Option%200 (Math|Vector|MakeVector (- (* _z (* (Math|Trig|Sin(Radians) (Math|Trig|DegreesToRadians (+ (- (* _index (/ (Variables|Default|GetSpread) (Variables|Default|GetProjectilesPerShot))) (/ (Variables|Default|GetSpread) 2.0)) 1.8e+02))) -1.0)) (* (Math|Trig|Cos(Radians) (Math|Trig|DegreesToRadians (+ (- (* _index (/ (Variables|Default|GetSpread) (Variables|Default|GetProjectilesPerShot))) (/ (Variables|Default|GetSpread) 2.0)) 1.8e+02))) _x)) _y (+ (* _x (Math|Trig|Sin(Radians) (Math|Trig|DegreesToRadians (+ (- (* _index (/ (Variables|Default|GetSpread) (Variables|Default|GetProjectilesPerShot))) (/ (Variables|Default|GetSpread) 2.0)) 1.8e+02)))) (* _z (* (Math|Trig|Cos(Radians) (Math|Trig|DegreesToRadians (+ (- (* _index (/ (Variables|Default|GetSpread) (Variables|Default|GetProjectilesPerShot))) (/ (Variables|Default|GetSpread) 2.0)) 1.8e+02))) -1.0)))) :Option%201 (Math|Vector|RotateVector Direction (Math|Rotator|MakeRotator 0.0 (Math|Random|RandomFloatinRange (* _spread -1.0) (* _spread 1.0)) 0.0))) (Variables|Default|GetNumProbes) (Math|Float|Round (* (Math|Conversions|ToFloat(Integer) (Variables|Default|GetBloodQuantity)) (Variables|/Game/Blueprints/Entities/Entity.Entity_C|GetPowerMultiplier _asentity) (Variables|/Game/Blueprints/Entities/Entity.Entity_C|GetSprayMultiplier _asentity))) (Math|Float|Round (* (Math|Conversions|ToFloat(Integer) (Variables|Default|GetProbeLifetime)) (Variables|/Game/Blueprints/Entities/Entity.Entity_C|GetPowerMultiplier _asentity) (Variables|/Game/Blueprints/Entities/Entity.Entity_C|GetSprayMultiplier _asentity))) (Variables|Default|GetProbeVariance) (Math|Float|Round (* (Math|Conversions|ToFloat(Integer) (Variables|Default|GetProbeSpeed)) (Variables|/Game/Blueprints/Entities/Entity.Entity_C|GetPowerMultiplier _asentity) (Variables|/Game/Blueprints/Entities/Entity.Entity_C|GetSprayMultiplier _asentity))) (Variables|Default|GetMaxAngle) (Math|Float|Round (* (Math|Conversions|ToFloat(Integer) (Variables|Default|GetDamage)) (Variables|/Game/Blueprints/Entities/Entity.Entity_C|GetPowerMultiplier _asentity) (Variables|/Game/Blueprints/Entities/Entity.Entity_C|GetDamageMultiplier _asentity))) 0))
        (Audio|PlaySoundatLocation (Variables|Default|GetSound) _returnvalue_9 "0, 0, 0" 1.0 1.0 0.0 0 0 0 0)
        (Variables|Default|SetAmmo (Math|Integer|Max(Integer) (- (Variables|Default|GetAmmo) (Variables|Default|GetAmmoPerShot))))
        (for _array_element (Variables|Default|GetAuras)
          (Game|AddComponentbyClass _returnvalue_10 _array_element))
        (else
          (Development|PrintString "Gun Out Of Ammo"))))))