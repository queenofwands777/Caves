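; Sword weapon sprite component that shows a katana and performs attacks in the X-Z plane.
; FireWeapon spawns a Swing actor offset from the owner along the aim direction and pitched to it.
; The next Tick ends the swing at once, snapping "hand"-tagged spring arms alternately to either side; timed rotation logic is disconnected.
; EndPlay resets those arms to zero rotation.
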(event EventBeginPlay
  (CallFunction|SetSprite "/Game/Assets/Weapons/Katana_Sprite.Katana_Sprite"))

(event EventEndPlay
  (params (EndPlayReason :type EEndPlayReason%20Enum :default "Destroyed"))
  (for _array_element (Actor|GetComponentsbyTag (Components|GetOwner) "/Script/Engine.SpringArmComponent" "hand")
    (Transformation|SetRelativeRotation _array_element "0, 0, 0" false false)))

(event EventTick
  (params (DeltaSeconds :type Float%20%28single-precision%29))
  (if (Variables|Default|GetIsSwinging)
    (CallFunction|Swing)))

(fn FireWeapon
  (params (Direction :type Vector :default "0, 0, 0"))
  (bind _returnvalue (Components|GetOwner))
  (bind _returnvalue_2 (Transformation|GetActorLocation _returnvalue))
  (bind (_x _y _z) (Math|Vector|BreakVector _returnvalue_2))
  (Variables|Default|SetIsSwinging true)
  (bind _output_get (Variables|Default|SetSwingDirection Direction))
  (Game|SpawnActorfromClass "/Game/Blueprints/Swing.Swing_C" (Math|Transform|MakeTransform (+ (Math|Vector|MakeVector _x 3.0 _z) (* _output_get "11.000000,1.000000,11.000000")) (Math|Rotator|MakeRotator 0.0 (* (Math|Float|Sign(Float) (.Z (Math|Vector|BreakVector (Variables|Default|GetSwingDirection)))) (+ (* -9e+01 (Math|Float|Sign(Float) (.Z (Math|Vector|BreakVector (Variables|Default|GetSwingDirection))))) (Class|KismetMathLibrary|DegAcos (Math|Vector|DotProduct (Variables|Default|GetSwingDirection) "1.000000,0.000000,0.000000")) 0.0)) 0.0)) "Undefined" "MultiplyWithRoot" 0 0))

(fn Swing
  (Variables|Default|SetSwingLeft (not (Variables|Default|GetSwingLeft)))
  (CallFunction|EndSwing))

(fn EndSwing
  (Variables|Default|SetIsSwinging false)
  (Variables|Default|SetSwingDirection "0, 0, 0")
  (Variables|Default|SetSwingTime 0)
  (for _array_element (Actor|GetComponentsbyTag (Components|GetOwner) "/Script/Engine.SpringArmComponent" "hand")
    (if (Variables|Default|GetSwingLeft)
      (Transformation|SetRelativeLocationAndRotation _array_element "0, 0, 0" "45.000000,0.000000,0.000000" false false)
      (else
        (Transformation|SetRelativeLocationAndRotation _array_element "0, 0, 0" "-45.000000,0.000000,0.000000" false false)))))