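; BloodOnFeet is an actor component that leaves a trail of FootPrint actors behind its moving owner, apparently as bloody tracks.
; Each tick it accumulates the owner's travel distance and spawns a print at the owner's location whenever DistanceThreshold is exceeded.
; Prints are pitched along the movement direction in the XZ plane, with a tiny random offset.
; A step counter destroys the component once it exceeds Lifetime.
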(event EventBeginPlay
  (bind _returnvalue (Components|GetOwner))
  (bind _returnvalue_2 (Transformation|GetActorLocation _returnvalue))
  (Variables|Default|SetCurrentPosition _returnvalue_2)
  (Variables|Default|SetLastPosition _returnvalue_2))

(event EventTick
  (params (DeltaSeconds :type Float%20%28single-precision%29))
  (bind _returnvalue (Math|Random|RandomUnitVector))
  (bind _returnvalue_2 (Components|GetOwner))
  (bind _returnvalue_3 (Transformation|GetActorTransform _returnvalue_2))
  (bind _returnvalue_4 (/ _returnvalue "1000.000000,1.000000,1000.000000"))
  (bind (_x _y _z) (Math|Vector|BreakVector _returnvalue_4))
  (bind (_location _rotation _scale) (Math|Transform|BreakTransform _returnvalue_3))
  (bind _output_get (Variables|Default|SetLastPosition (Variables|Default|GetCurrentPosition)))
  (bind _output_get_2 (Variables|Default|SetCurrentPosition (Transformation|GetActorLocation (Components|GetOwner))))
  (bind _output_get_3 (Variables|Default|SetDistanceTraveled (+ (Math|Vector|Distance(Vector) _output_get _output_get_2) (Variables|Default|GetDistanceTraveled))))
  (if (> _output_get_3 (Variables|Default|GetDistanceThreshold))
    (Game|SpawnActorfromClass "/Game/Blueprints/Effects/FootPrint.FootPrint_C" (Math|Transform|MakeTransform _location (Math|Rotator|MakeRotator 0.0 (+ (Class|KismetMathLibrary|DegAtan2 (.Z (Math|Vector|BreakVector (Math|Vector|Normalize (+ (- (Variables|Default|GetCurrentPosition) (Variables|Default|GetLastPosition)) (Math|Vector|MakeVector _x 0.0 _z))))) (.X (Math|Vector|BreakVector (Math|Vector|Normalize (+ (- (Variables|Default|GetCurrentPosition) (Variables|Default|GetLastPosition)) (Math|Vector|MakeVector _x 0.0 _z)))))) -9e+01) 0.0) _scale) "Undefined" "MultiplyWithRoot" 0 0)
    (Variables|Default|SetDistanceTraveled 0.0)
    (bind _result (Math|Integer|IncrementInt (Variables|Default|GetSteps))
      (:%20%20
        (if (> _result (Variables|Default|GetLifetime))
          (Components|DestroyComponent))))))