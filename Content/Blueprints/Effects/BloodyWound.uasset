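; BloodyWound is a component that makes its owning actor periodically bleed, then removes itself.
; A tick counter spawns a BloodSplatter each time it exceeds BloodRate, using the owner's transform with Y pinned to 1.0.
; Each splatter gets fixed single-probe parameters and is triggered immediately.
; LifeTimer counts splatters rather than time, and the component destroys itself once that count exceeds Lifetime.
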(event EventBeginPlay)

(event EventTick
  (params (DeltaSeconds :type Float%20%28single-precision%29))
  (bind _returnvalue (Components|GetOwner))
  (bind _returnvalue_2 (Transformation|GetActorTransform _returnvalue))
  (bind (_location _rotation _scale) (Math|Transform|BreakTransform _returnvalue_2))
  (bind (_x _y _z) (Math|Vector|BreakVector _location))
  (bind _returnvalue_3 (Math|Vector|MakeVector _x 1.0 _z))
  (bind _result (Math|Integer|IncrementInt (Variables|Default|GetBloodTimer))
    (:%20%20
      (if (> _result (Variables|Default|GetBloodRate))
        (Math|Integer|IncrementInt (Variables|Default|GetLifeTimer)
          (:%20%20
            (bind _returnvalue_4 (Game|SpawnActorfromClass "/Script/Caves.BloodSplatter" (Math|Transform|MakeTransform _returnvalue_3 _rotation _scale) "Undefined" "MultiplyWithRoot" 0 0))
            (Class|BloodSplatter|InitParams _returnvalue_4 1 1 15.0 3 1 2 0 "0, 0, 0" _returnvalue_3)
            (Class|BloodSplatter|Splatter _returnvalue_4)
            (Variables|Default|SetBloodTimer 0)
            (if (> (Variables|Default|GetLifeTimer) (Variables|Default|GetLifetime))
              (Components|DestroyComponent))))))))