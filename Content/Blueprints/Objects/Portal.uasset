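; Level exit portal that opens once all enemies are gone and carries the player to the next floor.
; Tick polls for Enemy actors and, when none remain, switches the flipbook, plays a chime and sets Open.
; A player overlapping the open portal is flagged Advancing, then the TopDown game mode clears the level and generates one from the GameVar floor counter, which is incremented.
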(event OnComponentBeginOverlap(Sphere)
  (params (OverlappedComponent :type Primitive%20Component%20Object%20Reference) (OtherActor :type Actor%20Object%20Reference) (OtherComp :type Primitive%20Component%20Object%20Reference) (OtherBodyIndex :type Integer) (bFromSweep :type Boolean) (SweepResult :type Hit%20Result%20Structure%20%28by%20ref%29))
  (bind _asplayer (Utilities|Casting|CastToplayer OtherActor))
  (if (Variables|Default|GetOpen)
    (bind _astop_down (Utilities|Casting|CastToTopDown (Game|GetGameMode)))
    (Variables|/Game/Blueprints/Entities/player.player_C|SetAdvancing _asplayer true)
    (Default|ClearLevel _astop_down)
    (bind _asgame_var (Utilities|Casting|CastToGameVar (Game|GetGameInstance)))
    (bind _result (Math|Integer|IncrementInt (Variables|/Game/Blueprints/Engine/GameVar.GameVar_C|GetFloor _asgame_var))
      (:%20%20
        (Default|GenerateLevel _astop_down _result)))))

(event EventTick
  (params (DeltaSeconds :type Float%20%28single-precision%29))
  (bind _outactors (Actor|GetAllActorsOfClass "/Game/Blueprints/Entities/enemy.enemy_C"))
  (if (Math|Conversions|ToBoolean(Integer) (Class|KismetMathLibrary|AndIntInt (Math|Conversions|ToInteger(Boolean) (== (Utilities|Array|Length _outactors) 0)) (Math|Conversions|ToInteger(Boolean) (not (Variables|Default|GetOpen)))))
    (CallFunction|OpenPortal)))

(fn ConstructionScript)

(fn OpenPortal
  (Sprite|SetFlipbook (Variables|Default|GetPortalOpen) "/Game/Assets/Level/Portal/Open/PortalOpen.PortalOpen")
  (Audio|PlaySound2D "/Game/Assets/Sound/Objects/PortalChime.PortalChime" 1.0 1.0 0.0 0 0)
  (Variables|Default|SetOpen true))