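; Altar actor that spawns a perk pickup just above itself when play begins.
; It reads the PerksRemaining list from the GameVar game instance and spawns a random class from it, falling back to BreakfastPerkPickup when the list is empty.
; The pickup takes the altar's rotation and scale at a slightly offset location; the altar itself never removes the chosen perk from the list.
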(event EventBeginPlay
  (bind _returnvalue (Transformation|GetActorTransform))
  (bind (_location _rotation _scale) (Math|Transform|BreakTransform _returnvalue))
  (bind (_x _y _z) (Math|Vector|BreakVector _location))
  (bind _returnvalue_2 (+ _y 1.0))
  (bind _returnvalue_3 (+ 7.0 _z))
  (bind _returnvalue_4 (Math|Vector|MakeVector _x _returnvalue_2 _returnvalue_3))
  (bind _returnvalue_5 (Math|Transform|MakeTransform _returnvalue_4 _rotation _scale))
  (bind _asgame_var (Utilities|Casting|CastToGameVar (Game|GetGameInstance)))
  (if (== (Utilities|Array|Length (Variables|/Game/Blueprints/Engine/GameVar.GameVar_C|GetPerksRemaining _asgame_var)) 0)
    (Game|SpawnActorfromClass "/Game/Blueprints/Pickups/PerkPickups/BreakfastPerkPickup.BreakfastPerkPickup_C" _returnvalue_5 "Undefined" "MultiplyWithRoot" 0 0)
    (else
      (Game|SpawnActorfromClass (Utilities|Array|Get(acopy) (Variables|/Game/Blueprints/Engine/GameVar.GameVar_C|GetPerksRemaining _asgame_var) (Math|Random|RandomInteger (Utilities|Array|Length (Variables|/Game/Blueprints/Engine/GameVar.GameVar_C|GetPerksRemaining _asgame_var)))) _returnvalue_5 "Undefined" "MultiplyWithRoot" 0 0))))

(event Collision|EventActorBeginOverlap
  (params (OtherActor :type Actor%20Object%20Reference)))

(event EventTick
  (params (DeltaSeconds :type Float%20%28single-precision%29)))

(fn ConstructionScript)