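; OverlapBullet is a 2D projectile actor that travels in the XZ plane along its Direction at Speed.
; It nudges itself forward along Direction on BeginPlay, then moves with a swept world offset each Tick.
; When its Sphere begins overlapping any actor, it prints that actor and spawns a BloodSplatter just past it, pitched to the travel direction via signed arccosine.
; The bullet then destroys itself.
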(event OnComponentEndOverlap(Sphere)
  (params (OverlappedComponent :type Primitive%20Component%20Object%20Reference) (OtherActor :type Actor%20Object%20Reference) (OtherComp :type Primitive%20Component%20Object%20Reference) (OtherBodyIndex :type Integer)))

(event OnComponentBeginOverlap(Sphere)
  (params (OverlappedComponent :type Primitive%20Component%20Object%20Reference) (OtherActor :type Actor%20Object%20Reference) (OtherComp :type Primitive%20Component%20Object%20Reference) (OtherBodyIndex :type Integer) (bFromSweep :type Boolean) (SweepResult :type Hit%20Result%20Structure%20%28by%20ref%29))
  (bind _direction (Variables|Default|GetDirection))
  (bind (_x _y) (Math|Vector2D|BreakVector2D _direction))
  (bind _returnvalue (Math|Vector|MakeVector _x 0.0 _y))
  (Development|PrintText (Utilities|Text|ToText(Object) OtherActor))
  (Game|SpawnActorfromClass "/Game/Blueprints/unused/BloodSplatter.BloodSplatter_C" (Math|Transform|MakeTransform (+ "0.000000,-1.000000,0.000000" (+ (Transformation|GetActorLocation OtherActor) (* "10.000000,0.000000,10.000000" _returnvalue))) (Math|Rotator|MakeRotator 0.0 (+ 2.7e+02 (* (Class|KismetMathLibrary|DegAcos (Math|Vector|DotProduct _returnvalue "1.000000,0.000000,0.000000")) (Math|Float|Sign(Float) _y))) 0.0)) "Undefined" "MultiplyWithRoot" 0 0)
  (Actor|DestroyActor))

(event EventBeginPlay
  (bind _direction (Variables|Default|GetDirection))
  (bind _returnvalue (Math|Conversions|ToVector(Vector2D) _direction))
  (bind (_x _y) (Math|Vector|BreakVector _returnvalue))
  (Transformation|AddActorWorldOffset (* "30.000000,0.000000,30.000000" (Math|Vector|MakeVector _x 0.0 _y))))

(event EventTick
  (params (DeltaSeconds :type Float%20%28single-precision%29))
  (bind _direction (Variables|Default|GetDirection))
  (bind _returnvalue (Math|Conversions|ToVector(Vector2D) _direction))
  (bind (_x _y) (Math|Vector|BreakVector _returnvalue))
  (Transformation|AddActorWorldOffset (* DeltaSeconds (* (Math|Vector|MakeVector _x 0.0 _y) (Variables|Default|GetSpeed))) true))

(fn ConstructionScript)