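; WebLauncher is a weapon Blueprint in the unused folder that fires a Bullet in a given direction.
; FireWeapon spawns the Bullet at the owner's transform, passing along damage, spread angle, and probe and blood settings from its variables.
; A trailing cast of the owner to Player leads to no further logic, and BeginPlay and Tick are disabled stubs.
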(event EventBeginPlay
  (|CallParentFunction) ; This node is disabled and will not be called.\nDrag off pins to build functionality.
)

(event EventTick
  (params (DeltaSeconds :type Float%20%28single-precision%29))
  (|CallParentFunction DeltaSeconds) ; This node is disabled and will not be called.\nDrag off pins to build functionality.
)

(fn FireWeapon
  (params (Direction :type Vector :default "0, 0, 0"))
  (bind _returnvalue (Components|GetOwner))
  (Game|SpawnActorfromClass "/Game/Blueprints/Weapons/Projectiles/Bullet.Bullet_C" (Transformation|GetActorTransform _returnvalue) "Undefined" "MultiplyWithRoot" 0 Direction (Variables|Default|GetNumProbes) (Variables|Default|GetBloodQuantity) (Variables|Default|GetProbeLifetime) (Variables|Default|GetProbeVariance) (Variables|Default|GetProbeSpeed) (Variables|Default|GetMaxAngle) (Variables|Default|GetDamage) 0)
  (Utilities|Casting|CastToPlayer _returnvalue))