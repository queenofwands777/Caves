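; HitBullet is a projectile actor that flies in the X-Z plane and leaves blood where it hits.
; On BeginPlay it applies an impulse to its Sphere, mapping the 2D Direction onto X and Z and scaling by Speed.
; On any hit it spawns a BloodSplatter slightly ahead along Direction, pitched by a signed-arccosine angle, then destroys itself.
; It also prints that angle, apparently for debugging.
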(event Collision|EventHit
  (params (MyComp :type Primitive%20Component%20Object%20Reference) (Other :type Actor%20Object%20Reference) (OtherComp :type Primitive%20Component%20Object%20Reference) (bSelfMoved :type Boolean) (HitLocation :type Vector :default "0, 0, 0") (HitNormal :type Vector :default "0, 0, 0") (NormalImpulse :type Vector :default "0, 0, 0") (Hit :type Hit%20Result%20Structure%20%28by%20ref%29))
  (bind _direction (Variables|Default|GetDirection))
  (bind _direction_2 (Variables|Default|GetDirection))
  (bind _returnvalue (Math|Conversions|ToVector(Vector2D) _direction))
  (bind (_x _y) (Math|Vector2D|BreakVector2D _direction_2))
  (bind _returnvalue_2 (Math|Vector|MakeVector _x 0.0 _y))
  (bind (_x_2 _y_2) (Math|Vector|BreakVector _returnvalue))
  (bind _returnvalue_3 (Math|Float|Sign(Float) _y))
  (bind _returnvalue_4 (Math|Vector|DotProduct _returnvalue_2 "1.000000,0.000000,0.000000"))
  (bind _returnvalue_5 (Class|KismetMathLibrary|DegAcos _returnvalue_4))
  (bind _returnvalue_6 (* _returnvalue_5 _returnvalue_3))
  (bind _returnvalue_7 (+ 2.7e+02 _returnvalue_6))
  (Development|PrintText (Utilities|Text|ToText(Float) _returnvalue_7 "HalfToEven"))
  (Game|SpawnActorfromClass "/Game/Blueprints/unused/BloodSplatter.BloodSplatter_C" (Math|Transform|MakeTransform (+ (* (Math|Vector|MakeVector _x_2 0.0 _y_2) "10.000000,0.000000,10.000000") HitLocation) (Math|Rotator|MakeRotator 0.0 _returnvalue_7 0.0)) "Undefined" "MultiplyWithRoot" 0 0)
  (Actor|DestroyActor))

(event EventTick
  (params (DeltaSeconds :type Float%20%28single-precision%29)))

(event EventBeginPlay
  (bind _direction (Variables|Default|GetDirection))
  (bind _returnvalue (Math|Conversions|ToVector(Vector2D) _direction))
  (bind (_x _y) (Math|Vector|BreakVector _returnvalue))
  (Physics|AddImpulse (Variables|Default|GetSphere) (* (Math|Vector|MakeVector _x 0.0 _y) (Variables|Default|GetSpeed)) "None" false))

(fn ConstructionScript)