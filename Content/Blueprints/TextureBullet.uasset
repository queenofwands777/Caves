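; TextureBullet is a projectile actor that produces blood splatter when it hits something other than static world geometry.
; It nudges itself at spawn, then moves each tick with a swept offset along Direction at Speed.
; On sphere overlap it destroys itself, first spawning and triggering a BloodSplatter actor for non-WorldStatic hits.
; Its own Splatter function, which spawns BloodProbe actors, is not called within this Blueprint.
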(event OnComponentBeginOverlap(Sphere)
  (params (OverlappedComponent :type Primitive%20Component%20Object%20Reference) (OtherActor :type Actor%20Object%20Reference) (OtherComp :type Primitive%20Component%20Object%20Reference) (OtherBodyIndex :type Integer) (bFromSweep :type Boolean) (SweepResult :type Hit%20Result%20Structure%20%28by%20ref%29))
  (Development|PrintString (Utilities|GetDisplayName OtherActor))
  (if (== (Math|Conversions|ToInteger(Byte) (Utilities|Enum|LiteralenumECollisionChannel "ECC_WorldStatic")) (Math|Conversions|ToInteger(Byte) (Collision|GetCollisionObjectType OtherComp)))
    (Actor|DestroyActor)
    (else
      (bind _returnvalue (Game|SpawnActorfromClass "/Script/Caves.BloodSplatter" (Transformation|GetActorTransform) "Undefined" "MultiplyWithRoot" 0 0))
      (Class|BloodSplatter|InitParams _returnvalue 3 45.0 10 2 3 (Variables|Default|GetDirection) (Transformation|GetActorLocation))
      (Class|BloodSplatter|Splatter _returnvalue)
      (Actor|DestroyActor))))

(event EventBeginPlay
  (Transformation|AddActorWorldOffset (* "30.000000,0.000000,30.000000" (Variables|Default|GetDirection))))

(event EventTick
  (params (DeltaSeconds :type Float%20%28single-precision%29))
  (Transformation|AddActorWorldOffset (* DeltaSeconds (* (Variables|Default|GetDirection) (Variables|Default|GetSpeed))) true))

(fn ConstructionScript)

(fn Splatter
  (params (direction :type Vector) (num_probes :type Integer) (max_angle :type Float%20%28double-precision%29))
  (for _index (range 0 num_probes)
    (Game|SpawnActorfromClass "/Game/Blueprints/BloodProbe.BloodProbe_C" (Math|Conversions|ToTransform(Vector) (+ "0.000000,-1.000000,0.000000" (Transformation|GetActorLocation))) "Undefined" "MultiplyWithRoot" 0 direction 0)))