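; Swing is a short-lived Paper2D sprite actor that detects a hit, apparently for a melee attack.
; Overlapping a WorldStatic component sets HitMade, which blocks any later hit effect.
; Otherwise, the first overlap prints the other actor's name and spawns several BloodProbe actors slightly offset from the swing's location.
; Tick counts frames and destroys the actor once the count exceeds LifetimeMax.
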(event OnComponentBeginOverlap(PaperSprite)
  (params (OverlappedComponent :type Primitive%20Component%20Object%20Reference) (OtherActor :type Actor%20Object%20Reference) (OtherComp :type Primitive%20Component%20Object%20Reference) (OtherBodyIndex :type Integer) (bFromSweep :type Boolean) (SweepResult :type Hit%20Result%20Structure%20%28by%20ref%29))
  (if (== (Math|Conversions|ToInteger(Byte) (Collision|GetCollisionObjectType OtherComp)) (Math|Conversions|ToInteger(Byte) (Utilities|Enum|LiteralenumECollisionChannel "ECC_WorldStatic")))
    (Variables|Default|SetHitMade true)
    (elif (not (Variables|Default|GetHitMade))
      (Development|PrintString (Utilities|GetDisplayName OtherActor))
      (for _index (range 0 3)
        (Game|SpawnActorfromClass "/Game/Blueprints/BloodProbe.BloodProbe_C" (Math|Conversions|ToTransform(Vector) (+ "0.000000,-2.000000,0.000000" (Transformation|GetActorLocation))) "Undefined" "MultiplyWithRoot" 0 "0.000000,0.000000,0.000000" 0)
        (Variables|Default|SetHitMade true)))))

(event EventTick
  (params (DeltaSeconds :type Float%20%28single-precision%29))
  (Variables|Default|SetCurrentLifetime (+ 1.0 (Variables|Default|GetCurrentLifetime)))
  (if (> (Variables|Default|GetCurrentLifetime) (Variables|Default|GetLifetimeMax))
    (Actor|DestroyActor)))

(fn ConstructionScript)