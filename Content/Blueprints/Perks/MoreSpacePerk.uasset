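; A perk Blueprint that grants the player one extra weapon slot.
; On BeginPlay it runs the parent logic, then, if Pickup is set, casts the game instance to StaticVariables and increments PlayerMaxWeapons.
; It prints a message confirming the increase, and its Tick is disabled.
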(event EventBeginPlay
  (|CallParentFunction)
  (if (Variables|Default|GetPickup)
    (bind _asstatic_variables (Utilities|Casting|CastToStaticVariables (Game|GetGameInstance)))
    (Variables|/Game/Blueprints/Engine/StaticVariables.StaticVariables_C|SetPlayerMaxWeapons _asstatic_variables (+ (Variables|/Game/Blueprints/Engine/StaticVariables.StaticVariables_C|GetPlayerMaxWeapons _asstatic_variables) 1))
    (Development|PrintString "Weaponslots increased")))

(event EventTick
  (params (DeltaSeconds :type Float%20%28single-precision%29))
  (|CallParentFunction DeltaSeconds) ; This node is disabled and will not be called.\nDrag off pins to build functionality.
)