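; Perk that heals its owning Player by absorbing blood splatters while they stand on blood.
; Each Tick checks OnBlood; below max health, it tints the sprite green and calls AbsorbSplatter on overlapping splatters.
; The absorbed amount, scaled down, heals player pawn 0 up to the GameInstance's dynamic max.
; Leaving blood restores a white tint; a timed-effect version remains as unconnected logic.
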(event EventBeginPlay)

(event EventTick
  (params (DeltaSeconds :type Float%20%28single-precision%29))
  (bind _asplayer (Utilities|Casting|CastToPlayer (Components|GetOwner)))
  (if (Variables|/Game/Blueprints/Entities/Entity.Entity_C|GetOnBlood _asplayer)
    (bind _asplayer_2 (Utilities|Casting|CastToPlayer (Components|GetOwner)))
    (CallFunction|SetonBlood _asplayer_2)
    (else
      (bind _asplayer_3 (Utilities|Casting|CastToPlayer (Components|GetOwner)))
      (CallFunction|SetOffBlood _asplayer_3))))

(fn SetonBlood
  (params (Player :type Player%20Object%20Reference))
  (if (< (Variables|/Game/Blueprints/Entities/Entity.Entity_C|GetHealth Player) (Variables|/Game/Blueprints/Engine/StaticVariables.StaticVariables_C|GetDynamicPlayerMaxHealth (.AsStatic%20Variables (Utilities|Casting|CastToStaticVariables (Game|GetGameInstance)))))
    (Sprite|SetSpriteColor (Variables|/Script/Paper2D.PaperCharacter|GetSprite Player) "(R=0.005173,G=1.000000,B=0.000000,A=1.000000)")
    (for _array_element (Collision|GetOverlappingActors (Variables|/Game/Blueprints/Entities/Entity.Entity_C|GetBloodCollider Player) "/Script/Caves.BloodSplatter" :!class /Script/Engine.PrimitiveComponent)
      (bind _asblood_splatter (Utilities|Casting|CastToBloodSplatter _array_element))
      (bind _returnvalue (Class|BloodSplatter|AbsorbSplatter _asblood_splatter (Transformation|GetActorLocation Player)))
      (bind _asplayer (Utilities|Casting|CastToPlayer (Game|Player|GetPlayerPawn 0)))
      (bind _asstatic_variables (Utilities|Casting|CastToStaticVariables (Game|GetGameInstance)))
      (Variables|/Game/Blueprints/Entities/Entity.Entity_C|SetHealth _asplayer (Math|Float|Min(Float) (Variables|/Game/Blueprints/Engine/StaticVariables.StaticVariables_C|GetDynamicPlayerMaxHealth _asstatic_variables) (+ (Variables|/Game/Blueprints/Entities/Entity.Entity_C|GetHealth _asplayer) (/ (Math|Conversions|ToFloat(Integer) _returnvalue) 1e+02)))))))

(fn SetOffBlood
  (params (Player :type Player%20Object%20Reference))
  (Sprite|SetSpriteColor (Variables|/Script/Paper2D.PaperCharacter|GetSprite Player) "(R=1.000000,G=1.000000,B=1.000000,A=1.000000)"))