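; Blood speed perk attached to the player that grants a modest speed boost while the player is on blood.
; Every tick it reads the owning Player's OnBlood flag and uses EffectActive to apply changes only on transitions.
; SetOnBlood raises SpeedMultiplier and tints the sprite orange, and SetOffBlood restores normal speed and white color.
; Timer-based expiry and refresh logic is present but disconnected, so the effect ends as soon as OnBlood clears.
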(event EventBeginPlay)

(event EventTick
  (params (DeltaSeconds :type Float%20%28single-precision%29))
  (bind _asplayer (Utilities|Casting|CastToPlayer (Components|GetOwner)))
  (if (Variables|/Game/Blueprints/Entities/Entity.Entity_C|GetOnBlood _asplayer)
    (if (not (Variables|Default|GetEffectActive))
      (CallFunction|SetonBlood (.AsPlayer (Utilities|Casting|CastToPlayer (Components|GetOwner))))
      (Variables|Default|SetEffectActive true))
    (elif (Variables|Default|GetEffectActive)
      (CallFunction|SetOffBlood (.AsPlayer (Utilities|Casting|CastToPlayer (Components|GetOwner))))
      (Variables|Default|SetEffectActive false))))

(fn SetonBlood
  (params (Player :type Player%20Object%20Reference))
  (Sprite|SetSpriteColor (Variables|/Script/Paper2D.PaperCharacter|GetSprite Player) "(R=1.000000,G=0.650098,B=0.000000,A=1.000000)")
  (Variables|/Game/Blueprints/Entities/Entity.Entity_C|SetSpeedMultiplier Player 1.2))

(fn SetOffBlood
  (params (Player :type Player%20Object%20Reference))
  (Sprite|SetSpriteColor (Variables|/Script/Paper2D.PaperCharacter|GetSprite Player) "(R=1.000000,G=1.000000,B=1.000000,A=1.000000)")
  (Variables|/Game/Blueprints/Entities/Entity.Entity_C|SetSpeedMultiplier Player 1.0))