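; Perk component for the Player that doubles damage while the player stands on blood.
; Every tick it reads the owner's OnBlood flag and calls SetOnBlood or SetOffBlood, which set the damage multiplier and tint the sprite red or restore white.
; An unconnected timed-effect version, with a lifetime counter that refreshes on reactivation, remains in the graph but never runs.
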(event EventBeginPlay)

(event EventTick
  (params (DeltaSeconds :type Float%20%28single-precision%29))
  (bind _asplayer (Utilities|Casting|CastToPlayer (Components|GetOwner)))
  (if (Variables|/Game/Blueprints/Entities/Entity.Entity_C|GetOnBlood _asplayer)
    (bind _asplayer_2 (Utilities|Casting|CastToPlayer (Components|GetOwner)))
    (CallFunction|SetonBlood _asplayer_2)
    (else
      (bind _asplayer_3 (Utilities|Casting|CastToPlayer (Components|GetOwner)))
      (CallFunction|SetOffBlood _asplayer_3))))

(fn SetonBlood
  (params (Player :type Player%20Object%20Reference))
  (Sprite|SetSpriteColor (Variables|/Script/Paper2D.PaperCharacter|GetSprite Player) "(R=1.000000,G=0.000000,B=0.000000,A=1.000000)")
  (Variables|/Game/Blueprints/Entities/Entity.Entity_C|SetDamageMultiplier Player 2.0))

(fn SetOffBlood
  (params (Player :type Player%20Object%20Reference))
  (Sprite|SetSpriteColor (Variables|/Script/Paper2D.PaperCharacter|GetSprite Player) "(R=1.000000,G=1.000000,B=1.000000,A=1.000000)")
  (Variables|/Game/Blueprints/Entities/Entity.Entity_C|SetDamageMultiplier Player 1.0))