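; HealthUpPerk is a perk attached to the player that raises maximum health and refills current health.
; On BeginPlay, if its Pickup flag is set, it casts its owner to Player and the game instance to StaticVariables.
; It increases DynamicPlayerMaxHealth on the game instance by half its current value, then sets the player's Health to the new maximum.
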(event EventBeginPlay
  (if (Variables|Default|GetPickup)
    (bind _asplayer (Utilities|Casting|CastToPlayer (Components|GetOwner)))
    (bind _asstatic_variables (Utilities|Casting|CastToStaticVariables (Game|GetGameInstance)))
    (bind _output_get (Variables|/Game/Blueprints/Engine/StaticVariables.StaticVariables_C|SetDynamicPlayerMaxHealth _asstatic_variables (+ (Variables|/Game/Blueprints/Engine/StaticVariables.StaticVariables_C|GetDynamicPlayerMaxHealth _asstatic_variables) (/ (Variables|/Game/Blueprints/Engine/StaticVariables.StaticVariables_C|GetDynamicPlayerMaxHealth _asstatic_variables) 2.0))))
    (Variables|/Game/Blueprints/Entities/Entity.Entity_C|SetHealth _asplayer _output_get)))

(event EventTick
  (params (DeltaSeconds :type Float%20%28single-precision%29))
  (|CallParentFunction DeltaSeconds) ; This node is disabled and will not be called.\nDrag off pins to build functionality.
)